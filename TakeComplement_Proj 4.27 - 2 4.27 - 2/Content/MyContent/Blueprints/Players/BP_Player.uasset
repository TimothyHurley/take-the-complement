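; Player vehicle pawn that drives among pedestrians, complimenting them to recharge its battery and build score, until an empty battery ends play.
; Each tick a camera line trace picks a pedestrian by interface and tag, updating crosshair, HUD prompts and custom-depth stencil outline.
; Clicking either compliments the target, making it follow and updating the range meter, or apologises to a stunned one, easing the throttle penalty that stunned pedestrians cause.
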(event EventBeginPlay
  (CallFunction|CreateHUD)
  (Variables|Default|SetIsPlaying? true)
  (Variables|/Script/Engine.PlayerController|SetbShowMouseCursor (Game|GetPlayerController 0) false))

(event EventTick
  (params (DeltaSeconds :type Float%20%28single-precision%29))
  (if (Variables|Default|GetIsPlaying?)
    (CallFunction|SetPlayerPositionandRotation)
    (if (Variables|/Game/MyContent/Blueprints/Widgets/HUD/W_Battery.W_Battery_C|GetIsEmpty? (Variables|/Game/MyContent/Blueprints/Widgets/HUD/W_HUD.W_HUD_C|GetW_Battery (Variables|Default|GetHUD_Ref)))
      (CallFunction|StopGameplayandCreateMenu)
      (else
        (bind (_returnvalue _hitactor) (CallFunction|GetTargetActor (Variables|Default|GetHUD_Ref)))
        (if (Variables|Default|GetIsCrosshairValid?)
          (CallFunction|IdentifyTargetActor _returnvalue _hitactor)
          (CallFunction|SetTargetPedestrian)
          (CallFunction|SetTargetPedestrianState)
          (CallFunction|SetCrosshairState (CallFunction|GetTargetPedestrianValidity))
          (CallFunction|SetTargetPedestrianOutline))))))

(event Input|AxisEvents|InputAxisMoveForward
  (params (AxisValue :type Float%20%28single-precision%29))
  (if (Variables|Default|GetIsPlayerStunned?)
    (Class|WheeledVehicleMovementComponent|SetThrottleInput (Variables|Default|GetVehicleMovement) (/ AxisValue (+ (* (Variables|Default|GetPedestrianNumberStunned) (Variables|Default|GetMovementSpeedDivisor)) 1.0)))
    (else
      (Class|WheeledVehicleMovementComponent|SetThrottleInput (Variables|Default|GetVehicleMovement) AxisValue))))

(event Input|AxisEvents|InputAxisMoveRight
  (params (AxisValue :type Float%20%28single-precision%29))
  (Class|WheeledVehicleMovementComponent|SetSteeringInput (Variables|Default|GetVehicleMovement) AxisValue))

(event Input|MouseEvents|LeftMouseButton
  (params (Key :type Key%20Structure :default "None"))
  (bind _targetpedestrian_ref (Variables|Default|GetTargetPedestrian_Ref))
  (:Pressed
    (if (CallFunction|GetTargetPedestrianValidity)
      (if (CallFunction|GetCrosshairValidity)
        (if (Variables|/Game/MyContent/Blueprints/Characters/BP_Pedestrian.BP_Pedestrian_C|GetIsStunned? (Variables|Default|GetTargetPedestrian_Ref))
          (CallFunction|ApologisetoPedestrian)
          (CallFunction|SetApologyPendingHidden)
          (Default|SetCorners (Variables|Default|GetHUD_Ref) (Variables|Default|GetPedestrianNumberStunned))
          (CallFunction|SetApologySentVisible)
          (Utilities|FlowControl|Delay 3.0)
          (CallFunction|SetApologySentHidden)
          (elif (not (Variables|/Game/MyContent/Blueprints/Characters/BP_Pedestrian.BP_Pedestrian_C|GetIsTooClose? (Variables|Default|GetTargetPedestrian_Ref)))
            (Variables|Default|SetIsPedestrianHighlighted? true)
            (Variables|/Game/MyContent/Blueprints/Characters/BP_Pedestrian.BP_Pedestrian_C|SetIsFollowingPlayer? _targetpedestrian_ref true)
            (Utilities|Array|Add (Variables|Default|GetPedestriansFollowing) _targetpedestrian_ref)
            (CallFunction|SetNearestPedestrianDistance (Math|Vector|Distance(Vector) (Transformation|GetActorLocation _targetpedestrian_ref) (Transformation|GetActorLocation self)))
            (CallFunction|SetPlayerBattery)
            (CallFunction|SetPlayerScoreCombo)
            (CallFunction|SetScoreStreakIsIncreasing)
            (CallFunction|SetComplementSentVisible)
            (Utilities|FlowControl|Delay 3.0)
            (CallFunction|SetComplementSentHidden)
            (else
              (Variables|Default|SetIsPedestrianHighlighted? false :!label _label)))))
      (else
        (goto _label)))))

(fn ConstructionScript
  (Variables|Default|SetNearestPedestrianDistance (Variables|Default|GetEscapeRange)))

(fn CreateHUD
  (bind _returnvalue (UserInterface|CreateWidget "/Game/MyContent/Blueprints/Widgets/HUD/W_HUD.W_HUD_C"))
  (bind _output_get (Variables|Default|SetHUD_Ref _returnvalue))
  (UserInterface|Viewport|AddtoViewport _output_get 0)
  (return))

(fn StopGameplayandCreateMenu
  (bind _vehiclemovement (Variables|Default|GetVehicleMovement))
  (Utilities|FlowControl|DoOnce false
    (:Completed
      (Input|DisableInput self (Game|GetPlayerController 0))
      (Class|WheeledVehicleMovementComponent|SetSteeringInput _vehiclemovement 0.0)
      (Class|WheeledVehicleMovementComponent|SetThrottleInput _vehiclemovement 0.0)
      (bind _outactors (Actor|GetAllActorsOfClass "/Game/MyContent/Blueprints/Characters/BP_Pedestrian.BP_Pedestrian_C"))
      (for _array_element _outactors
        (Default|ResettoFollowStreet _array_element true))
      (Variables|/Game/MyContent/Blueprints/Widgets/HUD/W_Timer.W_Timer_C|SetIsGameOver? (Variables|/Game/MyContent/Blueprints/Widgets/HUD/W_Scoreboard.W_Scoreboard_C|GetW_Timer (Variables|/Game/MyContent/Blueprints/Widgets/HUD/W_HUD.W_HUD_C|GetW_Scoreboard (Variables|Default|GetHUD_Ref))) true)
      (Variables|Default|SetIsPlaying? false)
      (bind _returnvalue (UserInterface|CreateWidget "/Game/MyContent/Blueprints/Widgets/Menu/W_Menu_Thanks.W_Menu_Thanks_C"))
      (UserInterface|Viewport|AddtoViewport _returnvalue 1)
      (return))))

(fn SetAudioInput
  (Audio|Parameter|SetFloatParameter (Variables|Default|GetEngineSound) "RPM" (Math|Float|Absolute(Float) (Class|WheeledVehicleMovementComponent|GetForwardSpeed (Variables|Default|GetVehicleMovement))) :!class /Script/Engine.AudioComponent))

(fn SetPlayerPositionandRotation
  (bind _camera (Variables|Components|GetCamera))
  (bind _relativerotation (Variables|/Script/Engine.SceneComponent|GetRelativeRotation _camera))
  (bind (_roll _pitch _yaw) (Math|Rotator|BreakRotator _relativerotation))
  (Variables|Default|SetIsReversing? (< (Class|WheeledVehicleMovementComponent|GetCurrentGear (Variables|Default|GetVehicleMovement)) 0))
  (Transformation|SetRelativeRotation (Variables|Components|GetCamera) (Math|Rotator|MakeRotator 0.0 (Math|Float|ClampAngle (+ (Input|AxisValues|GetLookUp) _pitch) -9e+01 9e+01) (+ (Input|AxisValues|GetLookRight) _yaw)) false false)
  (return))

(fn ApologisetoPedestrian
  (Utilities|FlowControl|DoOnce false
    (:Completed
      (bind _result (Math|Integer|DecrementInt (Variables|Default|GetPedestrianNumberStunned))
        (:%20%20
          (if (<= _result 0)
            (Variables|Default|SetPedestrianNumberStunned 0)
            (Variables|Default|SetIsPlayerStunned? false)
            (Default|SetCorners (Variables|Default|GetHUD_Ref)))
          (Variables|/Game/MyContent/Blueprints/Characters/BP_Pedestrian.BP_Pedestrian_C|SetIsStunned? (Variables|Default|GetTargetPedestrian_Ref) false)
          (if (Collision|IsOverlappingActor (Variables|Character|GetMesh) (Variables|Default|GetTargetPedestrian_Ref) :!class /Script/Engine.PrimitiveComponent)
            (Variables|/Game/MyContent/Blueprints/Characters/BP_Pedestrian.BP_Pedestrian_C|SetIsTooClose? (Variables|Default|GetTargetPedestrian_Ref) true))
          (return))))))

(fn SetPlayerBattery
  (bind _targetpedestrian_ref (Variables|Default|GetTargetPedestrian_Ref))
  (if (and (Variables|/Game/MyContent/Blueprints/Characters/BP_Pedestrian.BP_Pedestrian_C|GetIsFollowingPlayer? _targetpedestrian_ref) (not (Variables|/Game/MyContent/Blueprints/Characters/BP_Pedestrian.BP_Pedestrian_C|GetIsComplemented? _targetpedestrian_ref)))
    (Default|IncreaseBatteryPercentage (Variables|/Game/MyContent/Blueprints/Widgets/HUD/W_HUD.W_HUD_C|GetW_Battery (Variables|Default|GetHUD_Ref)))
    (Variables|/Game/MyContent/Blueprints/Characters/BP_Pedestrian.BP_Pedestrian_C|SetIsComplemented? (Variables|Default|GetTargetPedestrian_Ref) true))
  (return))

(fn SetPlayerScoreCombo
  (if (not (Variables|/Game/MyContent/Blueprints/Characters/BP_Pedestrian.BP_Pedestrian_C|GetIsAddedToScoreCombo? (Variables|Default|GetTargetPedestrian_Ref)))
    (Math|Integer|IncrementInt (Variables|/Game/MyContent/Blueprints/Widgets/HUD/W_Scoreboard_Combo.W_Scoreboard_Combo_C|GetScoreCombo (Variables|/Game/MyContent/Blueprints/Widgets/HUD/W_HUD.W_HUD_C|GetW_Scoreboard_Combo (Variables|Default|GetHUD_Ref)))
      (:%20%20
        (Variables|/Game/MyContent/Blueprints/Characters/BP_Pedestrian.BP_Pedestrian_C|SetIsAddedToScoreCombo? (Variables|Default|GetTargetPedestrian_Ref) true)
        (Widget|SetVisibility (Variables|/Game/MyContent/Blueprints/Widgets/HUD/W_HUD.W_HUD_C|GetW_Scoreboard_Combo (Variables|Default|GetHUD_Ref)) "Visible"))))
  (return))

(fn SetScoreStreakIsIncreasing
  (bind _hud_ref (Variables|Default|GetHUD_Ref))
  (bind _w_scoreboard (Variables|/Game/MyContent/Blueprints/Widgets/HUD/W_HUD.W_HUD_C|GetW_Scoreboard _hud_ref))
  (bind _w_scoreboard_streak (Variables|/Game/MyContent/Blueprints/Widgets/HUD/W_Scoreboard.W_Scoreboard_C|GetW_Scoreboard_Streak _w_scoreboard))
  (if (Variables|/Game/MyContent/Blueprints/Widgets/HUD/W_Scoreboard_Streak.W_Scoreboard_Streak_C|GetIsIncreasing? (Variables|/Game/MyContent/Blueprints/Widgets/HUD/W_Scoreboard.W_Scoreboard_C|GetW_Scoreboard_Streak (Variables|/Game/MyContent/Blueprints/Widgets/HUD/W_HUD.W_HUD_C|GetW_Scoreboard (Variables|Default|GetHUD_Ref))))
    _
    (else
      (Variables|/Game/MyContent/Blueprints/Widgets/HUD/W_Scoreboard_Streak.W_Scoreboard_Streak_C|SetIsIncreasing? _w_scoreboard_streak true)
      (Widget|SetVisibility _w_scoreboard_streak "Visible")))
  (return))

(fn GetTargetActor
  (params (HUD_Ref :type W%20HUD%20Object%20Reference))
  (bind _camera (Variables|Components|GetCamera))
  (bind _returnvalue (Transformation|GetWorldLocation _camera))
  (Variables|/Game/MyContent/Blueprints/Widgets/HUD/W_HUD.W_HUD_C|GetW_Crosshair HUD_Ref
    (:then
      (Variables|Default|SetIsCrosshairValid? true)
      (bind (_outhit _returnvalue_2) (Collision|LineTraceByChannel _returnvalue (+ _returnvalue (* (Math|Vector|GetForwardVector _camera) (Variables|Default|GetComplementRange))) "TraceTypeQuery2" false 0 "None")))
    (:else
      (Variables|Default|SetIsCrosshairValid? false)))
  (return _returnvalue_2 (.HitActor (Collision|BreakHitResult _outhit))))

(fn IdentifyTargetActor
  (params (ReturnValue :type Boolean) (HitActor :type Actor%20Object%20Reference))
  (if ReturnValue
    (if (Utilities|DoesObjectImplementInterface HitActor "/Game/MyContent/Blueprints/Interfaces/BP_ComplementInterface.BP_ComplementInterface_C")
      (Variables|Default|SetPedestrianID_Ref (Utilities|Array|Get(acopy) (Variables|/Script/Engine.Actor|GetTags HitActor)))
      (Variables|Default|SetIsInComplementRange? true)
      (else
        (Variables|Default|SetPedestrianID_Ref "None" :!label _label)
        (Variables|Default|SetIsInComplementRange? false)))
    (else
      (goto _label)))
  (return))

(fn SetTargetPedestrian
  (for _array_element (Variables|Default|GetPedestrian_Refs)
    (Variables|/Game/MyContent/Blueprints/Characters/BP_Pedestrian.BP_Pedestrian_C|SetIsTargetReference? _array_element false))
  (if (Variables|Default|GetIsInComplementRange?)
    (bind _array_element_2 (Utilities|Array|ForEachLoopwithBreak (Variables|Default|GetPedestrian_Refs) :!label _label)
      (:LoopBody
        (if (Utilities|Name|Equal(Name) (Utilities|Array|Get(acopy) (Variables|/Script/Engine.Actor|GetTags _array_element_2)) (Variables|Default|GetPedestrianID_Ref))
          (bind _output_get (Variables|Default|SetTargetPedestrian_Ref _array_element_2))
          (Variables|/Game/MyContent/Blueprints/Characters/BP_Pedestrian.BP_Pedestrian_C|SetIsTargetReference? _output_get true)
          (goto _label Break)
          (else
            (Variables|Default|SetTargetPedestrian_Ref 0)
            (Variables|/Game/MyContent/Blueprints/Characters/BP_Pedestrian.BP_Pedestrian_C|SetIsTargetReference? _array_element_2 false))))
      (:Completed
        (return)))
    (else
      (return))))

(fn SetCrosshairState
  (params (IsValid? :type Boolean))
  (if IsValid?
    (if (not (Utilities|Name|Equal(Name) (Variables|Default|GetPedestrianID_Ref) "None"))
      (if (Variables|/Game/MyContent/Blueprints/Characters/BP_Pedestrian.BP_Pedestrian_C|GetIsTooClose? (Variables|Default|GetTargetPedestrian_Ref))
        (if (CallFunction|GetCrosshairValidity)
          _
          (else
            (UserInterface|Viewport|AddtoViewport (Variables|/Game/MyContent/Blueprints/Widgets/HUD/W_HUD.W_HUD_C|GetW_Crosshair (Variables|Default|GetHUD_Ref)) 0)))
        (elif (CallFunction|GetCrosshairValidity)
          _
          (else
            (UserInterface|Viewport|AddtoViewport (Variables|/Game/MyContent/Blueprints/Widgets/HUD/W_HUD.W_HUD_C|GetW_Crosshair (Variables|Default|GetHUD_Ref)) 0))))
      (else
        (if (CallFunction|GetCrosshairValidity) :!label _label
          (Widget|RemovefromParent (Variables|/Game/MyContent/Blueprints/Widgets/HUD/W_HUD.W_HUD_C|GetW_Crosshair (Variables|Default|GetHUD_Ref))))))
    (else
      (goto _label)))
  (return))

(fn SetTargetPedestrianState
  (bind _targetpedestrian_ref (Variables|Default|GetTargetPedestrian_Ref))
  (if (CallFunction|GetTargetPedestrianValidity)
    (if (Variables|/Game/MyContent/Blueprints/Characters/BP_Pedestrian.BP_Pedestrian_C|GetIsStunned? (Variables|Default|GetTargetPedestrian_Ref))
      (Variables|Default|SetOutlineStencilValue 4)
      (Default|SetStunned (Variables|/Game/MyContent/Blueprints/Widgets/HUD/W_HUD.W_HUD_C|GetW_Prompt_Complement (Variables|Default|GetHUD_Ref)))
      (if (CallFunction|GetCrosshairValidity)
        (CallFunction|SetApologyPendingVisible)
        (else
          (CallFunction|SetApologyPendingHidden)
          (Default|SetOutOfRange (Variables|/Game/MyContent/Blueprints/Widgets/HUD/W_HUD.W_HUD_C|GetW_Prompt_Complement (Variables|Default|GetHUD_Ref)))))
      (elif (Variables|/Game/MyContent/Blueprints/Characters/BP_Pedestrian.BP_Pedestrian_C|GetIsFollowingPlayer? (Variables|Default|GetTargetPedestrian_Ref))
        (Variables|Default|SetOutlineStencilValue 3)
        (Default|SetFollowing (Variables|/Game/MyContent/Blueprints/Widgets/HUD/W_HUD.W_HUD_C|GetW_Prompt_Complement (Variables|Default|GetHUD_Ref)))
        (elif (CallFunction|GetCrosshairValidity)
          (if (Variables|/Game/MyContent/Blueprints/Characters/BP_Pedestrian.BP_Pedestrian_C|GetIsTooClose? (Variables|Default|GetTargetPedestrian_Ref))
            _
            (else
              _))
          (Variables|Default|SetOutlineStencilValue 1)
          (Default|SetinRange (Variables|/Game/MyContent/Blueprints/Widgets/HUD/W_HUD.W_HUD_C|GetW_Prompt_Complement (Variables|Default|GetHUD_Ref)))
          (CallFunction|SetComplementPendingVisible)
          (elif (not (and (Variables|/Game/MyContent/Blueprints/Characters/BP_Pedestrian.BP_Pedestrian_C|GetIsStunned? _targetpedestrian_ref) (Variables|/Game/MyContent/Blueprints/Characters/BP_Pedestrian.BP_Pedestrian_C|GetIsFollowingPlayer? _targetpedestrian_ref)))
            (Variables|Default|SetOutlineStencilValue 0)
            (Default|SetOutOfRange (Variables|/Game/MyContent/Blueprints/Widgets/HUD/W_HUD.W_HUD_C|GetW_Prompt_Complement (Variables|Default|GetHUD_Ref)))
            (CallFunction|SetComplementPendingHidden))))))
  (return))

(fn SetTargetPedestrianOutline
  (bind _targetpedestrian_ref (Variables|Default|GetTargetPedestrian_Ref))
  (bind _targetpedestrian_ref_2 (Variables|Default|GetTargetPedestrian_Ref))
  (if (CallFunction|GetCrosshairValidity)
    (Rendering|SetCustomDepthStencilValue (Variables|/Script/Engine.Character|GetMesh _targetpedestrian_ref_2) (Variables|Default|GetOutlineStencilValue) :!label _label)
    (if (Variables|/Game/MyContent/Blueprints/Characters/BP_Pedestrian.BP_Pedestrian_C|GetIsStunned? _targetpedestrian_ref_2)
      (bind _output_get (Variables|Default|SetOutlineStencilValue 4))
      (Rendering|SetCustomDepthStencilValue (Variables|/Script/Engine.Character|GetMesh _targetpedestrian_ref) _output_get)
      (Components|Movement|StopMovementImmediately (Variables|/Script/Engine.Character|GetCharacterMovement _targetpedestrian_ref)))
    (elif (not (Utilities|Enum|Equal(Enum) (Utilities|GetDisplayName (Variables|Default|GetTargetPedestrian_Ref)) ""))
      (if (< (Variables|Default|GetOutlineStencilValue) 2)
        (goto _label)
        (else
          _))))
  (return))

(fn SetComplementPendingVisible
  (Rendering|Components|TextRender|SetText (Variables|/Game/MyContent/Blueprints/Widgets/HUD/W_Recipient_Complement.W_Recipient_Complement_C|GetTextBlock_Name (Variables|/Game/MyContent/Blueprints/Widgets/HUD/W_HUD.W_HUD_C|GetW_Recipient_Complement (Variables|Default|GetHUD_Ref))) (Variables|/Game/MyContent/Blueprints/Characters/BP_Pedestrian.BP_Pedestrian_C|GetPedestrianName (Variables|Default|GetTargetPedestrian_Ref)))
  (Widget|SetVisibility (Variables|/Game/MyContent/Blueprints/Widgets/HUD/W_HUD.W_HUD_C|GetW_Recipient_Complement (Variables|Default|GetHUD_Ref)) "Visible")
  (return))

(fn SetComplementPendingHidden
  (Widget|SetVisibility (Variables|/Game/MyContent/Blueprints/Widgets/HUD/W_HUD.W_HUD_C|GetW_Recipient_Complement (Variables|Default|GetHUD_Ref)) "Hidden")
  (return))

(fn SetComplementSentVisible
  (Rendering|Components|TextRender|SetText (Variables|/Game/MyContent/Blueprints/Widgets/HUD/W_Comment_Complement.W_Comment_Complement_C|GetTextBlock_Comment (Variables|/Game/MyContent/Blueprints/Widgets/HUD/W_HUD.W_HUD_C|GetW_Comment_Complement (Variables|Default|GetHUD_Ref))) (CallFunction|GetRandomTextValue (Variables|Default|GetComplements)))
  (Widget|SetVisibility (Variables|/Game/MyContent/Blueprints/Widgets/HUD/W_HUD.W_HUD_C|GetW_Comment_Complement (Variables|Default|GetHUD_Ref)) "Visible")
  (return))

(fn SetComplementSentHidden
  (Widget|SetVisibility (Variables|/Game/MyContent/Blueprints/Widgets/HUD/W_HUD.W_HUD_C|GetW_Comment_Complement (Variables|Default|GetHUD_Ref)) "Hidden")
  (return))

(fn SetApologyPendingVisible
  (Rendering|Components|TextRender|SetText (Variables|/Game/MyContent/Blueprints/Widgets/HUD/W_Recipient_Apology.W_Recipient_Apology_C|GetTextBlock_Name (Variables|/Game/MyContent/Blueprints/Widgets/HUD/W_HUD.W_HUD_C|GetW_Recipient_Apology (Variables|Default|GetHUD_Ref))) (Variables|/Game/MyContent/Blueprints/Characters/BP_Pedestrian.BP_Pedestrian_C|GetPedestrianName (Variables|Default|GetTargetPedestrian_Ref)))
  (Widget|SetVisibility (Variables|/Game/MyContent/Blueprints/Widgets/HUD/W_HUD.W_HUD_C|GetW_Recipient_Apology (Variables|Default|GetHUD_Ref)) "Visible")
  (return))

(fn SetApologyPendingHidden
  (Widget|SetVisibility (Variables|/Game/MyContent/Blueprints/Widgets/HUD/W_HUD.W_HUD_C|GetW_Recipient_Apology (Variables|Default|GetHUD_Ref)) "Hidden")
  (return))

(fn SetApologySentVisible
  (Rendering|Components|TextRender|SetText (Variables|/Game/MyContent/Blueprints/Widgets/HUD/W_Comment_Apology.W_Comment_Apology_C|GetTextBlock_Comment (Variables|/Game/MyContent/Blueprints/Widgets/HUD/W_HUD.W_HUD_C|GetW_Comment_Apology (Variables|Default|GetHUD_Ref))) (CallFunction|GetRandomTextValue (Variables|Default|GetApologies)))
  (Widget|SetVisibility (Variables|/Game/MyContent/Blueprints/Widgets/HUD/W_HUD.W_HUD_C|GetW_Comment_Apology (Variables|Default|GetHUD_Ref)) "Visible")
  (return))

(fn SetApologySentHidden
  (Widget|SetVisibility (Variables|/Game/MyContent/Blueprints/Widgets/HUD/W_HUD.W_HUD_C|GetW_Comment_Apology (Variables|Default|GetHUD_Ref)) "Hidden")
  (return))

(fn GetCrosshairValidity
  (if (UserInterface|Viewport|IsinViewport (Variables|/Game/MyContent/Blueprints/Widgets/HUD/W_HUD.W_HUD_C|GetW_Crosshair (Variables|Default|GetHUD_Ref)))
    (return true)
    (else
      (return false))))

(fn GetTargetPedestrianValidity
  (if (Utilities|Enum|Equal(Enum) (Utilities|GetDisplayName (Variables|Default|GetTargetPedestrian_Ref)) "")
    (Variables|Default|SetTargetPedestrian_Ref 0)
    (return false)
    (else
      (return true))))

(fn GetRandomTextValue
  (params (TextArray :type Array%20of%20Texts))
  (return (Utilities|Array|Get(acopy) TextArray (Math|Random|RandomInteger (Utilities|Array|Length TextArray)))))

(fn SetNearestPedestrianDistance
  (params (PedestrianDistance :type Float%20%28single-precision%29) (Pedestrian_Ref :type BP%20Pedestrian%20Object%20Reference))
  (bind _hud_ref (Variables|Default|GetHUD_Ref))
  (bind _hud_ref_2 (Variables|Default|GetHUD_Ref))
  (bind _hud_ref_3 (Variables|Default|GetHUD_Ref))
  (bind _escaperange (Variables|Default|GetEscapeRange))
  (bind _hud_ref_4 (Variables|Default|GetHUD_Ref))
  (bind _returnvalue (Math|Float|SafeDivide PedestrianDistance _escaperange))
  (bind _w_rangemeter (Variables|/Game/MyContent/Blueprints/Widgets/HUD/W_HUD.W_HUD_C|GetW_RangeMeter _hud_ref))
  (bind _w_rangemeter_2 (Variables|/Game/MyContent/Blueprints/Widgets/HUD/W_HUD.W_HUD_C|GetW_RangeMeter _hud_ref_2))
  (bind _w_rangemeter_3 (Variables|/Game/MyContent/Blueprints/Widgets/HUD/W_HUD.W_HUD_C|GetW_RangeMeter _hud_ref_3))
  (bind _w_rangemeter_4 (Variables|/Game/MyContent/Blueprints/Widgets/HUD/W_HUD.W_HUD_C|GetW_RangeMeter _hud_ref_4))
  (if (< (Variables|/Script/UMG.ProgressBar|GetPercent (Variables|/Game/MyContent/Blueprints/Widgets/HUD/W_RangeMeter.W_RangeMeter_C|GetRangeMeter_ProgressBar (Variables|/Game/MyContent/Blueprints/Widgets/HUD/W_HUD.W_HUD_C|GetW_RangeMeter (Variables|Default|GetHUD_Ref)))) _returnvalue)
    (LocalVariables|SetLowestPercent_Loc 1.0)
    (for _array_element (Variables|Default|GetPedestriansFollowing)
      (if (not (> (LocalVariables|GetLowestPercent_Loc) (Math|Float|SafeDivide (Math|Vector|Distance(Vector) (Transformation|GetActorLocation _array_element) (Transformation|GetActorLocation self)) (Variables|Default|GetEscapeRange))))
        (Utilities|Array|RemoveItem (Variables|Default|GetPedestriansFollowing) _array_element)
        (else
          (LocalVariables|SetLowestPercent_Loc (Math|Float|SafeDivide (Math|Vector|Distance(Vector) (Transformation|GetActorLocation _array_element) (Transformation|GetActorLocation self)) (Variables|Default|GetEscapeRange))))))
    (Progress|SetPercent (Variables|/Game/MyContent/Blueprints/Widgets/HUD/W_RangeMeter.W_RangeMeter_C|GetRangeMeter_ProgressBar (Variables|/Game/MyContent/Blueprints/Widgets/HUD/W_HUD.W_HUD_C|GetW_RangeMeter (Variables|Default|GetHUD_Ref))) (LocalVariables|GetLowestPercent_Loc))
    (if (> (LocalVariables|GetLowestPercent_Loc) 0.15)
      (Class|ProgressBar|SetFillColorandOpacity (Variables|/Game/MyContent/Blueprints/Widgets/HUD/W_RangeMeter.W_RangeMeter_C|GetRangeMeter_ProgressBar _w_rangemeter_2) (Utilities|Array|Get(acopy) (Variables|/Game/MyContent/Blueprints/Widgets/HUD/W_RangeMeter.W_RangeMeter_C|GetImageColours _w_rangemeter_2)))
      (else
        (Class|ProgressBar|SetFillColorandOpacity (Variables|/Game/MyContent/Blueprints/Widgets/HUD/W_RangeMeter.W_RangeMeter_C|GetRangeMeter_ProgressBar _w_rangemeter_3) (Utilities|Array|Get(acopy) (Variables|/Game/MyContent/Blueprints/Widgets/HUD/W_RangeMeter.W_RangeMeter_C|GetImageColours _w_rangemeter_3) 1))))
    (else
      (Progress|SetPercent (Variables|/Game/MyContent/Blueprints/Widgets/HUD/W_RangeMeter.W_RangeMeter_C|GetRangeMeter_ProgressBar (Variables|/Game/MyContent/Blueprints/Widgets/HUD/W_HUD.W_HUD_C|GetW_RangeMeter (Variables|Default|GetHUD_Ref))) _returnvalue)
      (if (> _returnvalue 0.15)
        (Class|ProgressBar|SetFillColorandOpacity (Variables|/Game/MyContent/Blueprints/Widgets/HUD/W_RangeMeter.W_RangeMeter_C|GetRangeMeter_ProgressBar _w_rangemeter) (Utilities|Array|Get(acopy) (Variables|/Game/MyContent/Blueprints/Widgets/HUD/W_RangeMeter.W_RangeMeter_C|GetImageColours _w_rangemeter)))
        (else
          (Class|ProgressBar|SetFillColorandOpacity (Variables|/Game/MyContent/Blueprints/Widgets/HUD/W_RangeMeter.W_RangeMeter_C|GetRangeMeter_ProgressBar _w_rangemeter_4) (Utilities|Array|Get(acopy) (Variables|/Game/MyContent/Blueprints/Widgets/HUD/W_RangeMeter.W_RangeMeter_C|GetImageColours _w_rangemeter_4) 1))))))
  (return))

(fn SetEscapeRangeBar
  (params (NearestPedestrianDistance :type Float%20%28single-precision%29))
  (bind _escaperange (Variables|Default|GetEscapeRange))
  (bind _hud_ref (Variables|Default|GetHUD_Ref))
  (bind _hud_ref_2 (Variables|Default|GetHUD_Ref))
  (bind _returnvalue (Math|Float|SafeDivide NearestPedestrianDistance _escaperange))
  (bind _w_rangemeter (Variables|/Game/MyContent/Blueprints/Widgets/HUD/W_HUD.W_HUD_C|GetW_RangeMeter _hud_ref))
  (bind _w_rangemeter_2 (Variables|/Game/MyContent/Blueprints/Widgets/HUD/W_HUD.W_HUD_C|GetW_RangeMeter _hud_ref_2))
  (bind _rangemeter_progressbar (Variables|/Game/MyContent/Blueprints/Widgets/HUD/W_RangeMeter.W_RangeMeter_C|GetRangeMeter_ProgressBar _w_rangemeter))
  (bind _rangemeter_progressbar_2 (Variables|/Game/MyContent/Blueprints/Widgets/HUD/W_RangeMeter.W_RangeMeter_C|GetRangeMeter_ProgressBar _w_rangemeter_2))
  (if (<= _returnvalue 1e+01)
    (Class|ProgressBar|SetFillColorandOpacity _rangemeter_progressbar_2 (Utilities|Array|Get(acopy) (Variables|/Game/MyContent/Blueprints/Widgets/HUD/W_RangeMeter.W_RangeMeter_C|GetImageColours _w_rangemeter_2) 1))
    (Progress|SetPercent _rangemeter_progressbar_2 _returnvalue)
    (else
      (Class|ProgressBar|SetFillColorandOpacity _rangemeter_progressbar (Utilities|Array|Get(acopy) (Variables|/Game/MyContent/Blueprints/Widgets/HUD/W_RangeMeter.W_RangeMeter_C|GetImageColours _w_rangemeter)))
      (Progress|SetPercent _rangemeter_progressbar _returnvalue)))
  (return))
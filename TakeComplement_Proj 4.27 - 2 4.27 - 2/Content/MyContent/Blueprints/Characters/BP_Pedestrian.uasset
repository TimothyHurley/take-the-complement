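; Pedestrian NPC with randomized mesh and speed that walks to a street target, then respawns via GM_Infinite, or chases the player while flagged as following.
; A looping timer selects stunned, follow or street movement, with DoOnce gates updating follower and HUD combo state on transitions.
; Bumping a non-follower stuns it and the player; nearby followers raise battery drain.
; Escaping followers' range lowers the combo, updating score at zero.
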(event OnComponentBeginOverlap(CapsuleComponent)
  (params (OverlappedComponent :type Primitive%20Component%20Object%20Reference) (OtherActor :type Actor%20Object%20Reference) (OtherComp :type Primitive%20Component%20Object%20Reference) (OtherBodyIndex :type Integer) (bFromSweep :type Boolean) (SweepResult :type Hit%20Result%20Structure%20%28by%20ref%29))
  (bind _player_ref (Variables|References|GetPlayer_Ref))
  (if (and (== OtherActor (Variables|References|GetPlayer_Ref)) (not (Variables|Bools|GetIsFollowingPlayer?)))
    (Utilities|FlowControl|DoOnce false
      (:Completed
        (CallFunction|SetStunnedVariables)
        (Default|PlayAnimations (Variables|References|GetHUD_Ref) (Variables|/Game/MyContent/Blueprints/Players/BP_Player.BP_Player_C|GetPedestrianNumberStunned _player_ref))
        (Default|SetFieldOfView _player_ref true)
        (Variables|/Game/MyContent/Blueprints/Players/BP_Player.BP_Player_C|SetIsComplementDisabled? (Variables|References|GetPlayer_Ref) true)
        (Utilities|FlowControl|Delay 2.25)
        (Variables|/Game/MyContent/Blueprints/Players/BP_Player.BP_Player_C|SetIsComplementDisabled? (Variables|References|GetPlayer_Ref) false)
        (Widget|SetVisibility (Variables|/Game/MyContent/Blueprints/Widgets/HUD/W_HUD.W_HUD_C|GetW_Crosshair_Disabled (Variables|References|GetHUD_Ref)) "Hidden")))))

(event OnComponentBeginOverlap(CollisionSphere_Thank)
  (params (OverlappedComponent :type Primitive%20Component%20Object%20Reference) (OtherActor :type Actor%20Object%20Reference) (OtherComp :type Primitive%20Component%20Object%20Reference) (OtherBodyIndex :type Integer) (bFromSweep :type Boolean) (SweepResult :type Hit%20Result%20Structure%20%28by%20ref%29))
  (if (and (== OtherActor (Variables|References|GetPlayer_Ref)) (Variables|Bools|GetIsFollowingPlayer?))
    (CallFunction|IncreaseBatteryReduceRate)))

(event OnComponentEndOverlap(CollisionSphere_Thank)
  (params (OverlappedComponent :type Primitive%20Component%20Object%20Reference) (OtherActor :type Actor%20Object%20Reference) (OtherComp :type Primitive%20Component%20Object%20Reference) (OtherBodyIndex :type Integer))
  (if (and (== OtherActor (Variables|References|GetPlayer_Ref)) (Variables|Bools|GetIsFollowingPlayer?))
    (CallFunction|DecreaseBatteryReduceRate)))

(event Custom|FollowPlayer
  (Utilities|FlowControl|Sequence
    (:then_0
      (AI|AIMoveTo self "0, 0, 0" (Variables|References|GetPlayer_Ref) 5.0 false
        (:then
          (if (not (CallFunction|GetDistancefromPlayer))
            (CallFunction|ResetFollowStreet false)))))
    (:then_1
      (Utilities|FlowControl|DoOnce false
        (:Completed
          (CallFunction|UpdatePedestriansFollowingPlayer true)
          (CallFunction|UpdatePedestrianCombo)
          (CallFunction|ResetDoOnceFollowStreet))))))

(event Custom|FollowStreet
  (Utilities|FlowControl|Sequence
    (:then_0
      (AI|AIMoveTo self (Variables|Default|GetTargetLocation) 0 1e+01 false
        (:OnSuccess
          (CallFunction|DestroySelf)
          (Default|SpawnPedestrian (Variables|References|GetGameMode_Ref)))))
    (:then_1
      (Utilities|FlowControl|DoOnce false
        (:Completed
          (CallFunction|UpdatePedestriansFollowingPlayer false)
          (CallFunction|ResetDoOnceFollowPlayer))))))

(event Custom|UpdateMovement
  (if (Variables|Bools|GetIsStunned?)
    (Components|Movement|StopMovementImmediately (Variables|Character|GetCharacterMovement))
    (Rendering|SetCustomDepthStencilValue (Variables|Character|GetMesh) 4)
    (elif (Variables|Bools|GetIsFollowingPlayer?)
      (CallFunction|FollowPlayer)
      (else
        (if (Variables|Bools|GetIsReferenced?)
          _
          (else
            (Rendering|SetCustomDepthStencilValue (Variables|Character|GetMesh) 0)))
        (CallFunction|FollowStreet)))))

(event Custom|ResetDoOnce_FollowPlayer
  (Utilities|FlowControl|DoOnce false) ; enters at Reset
)

(event Custom|ResetDoOnce_FollowStreet
  (Utilities|FlowControl|DoOnce false) ; enters at Reset
)

(event Custom|ResetDoOnce_Stun
  (bind _player_ref (Variables|References|GetPlayer_Ref))
  (Utilities|FlowControl|DoOnce false) ; enters at Reset
)

(event EventBeginPlay
  (Utilities|FlowControl|Delay 0.2)
  (CallFunction|SetReferences)
  (Utilities|Time|SetTimerbyEvent (delegate Custom|UpdateMovement) 0.1 true))

(fn ConstructionScript
  (bind _charactermodels (Variables|References|GetCharacterModels))
  (bind _charactermovement (Variables|Character|GetCharacterMovement))
  (Class|SkinnedMeshComponent|SetSkeletalMesh (Variables|Character|GetMesh) (Utilities|Array|Get(acopy) _charactermodels (Math|Random|RandomIntegerinRange 0 (Utilities|Array|Length _charactermodels))) true)
  (Variables|/Script/Engine.CharacterMovementComponent|SetMaxWalkSpeed _charactermovement (Math|Random|RandomFloatinRange (- (Variables|/Script/Engine.CharacterMovementComponent|GetMaxWalkSpeed _charactermovement) 15.0) (+ (Variables|/Script/Engine.CharacterMovementComponent|GetMaxWalkSpeed _charactermovement) 15.0))))

(fn SetReferences
  (bind _returnvalue (Actor|GetActorOfClass "/Game/MyContent/Blueprints/GameModes/GM_Infinite.GM_Infinite_C"))
  (Variables|References|SetGameMode_Ref _returnvalue)
  (bind _returnvalue_2 (Actor|GetActorOfClass "/Game/MyContent/Blueprints/Players/BP_Player.BP_Player_C"))
  (Variables|References|SetPlayer_Ref _returnvalue_2)
  (bind _foundwidgets (Widget|GetAllWidgetsOfClass "/Game/MyContent/Blueprints/Widgets/HUD/W_HUD.W_HUD_C" true))
  (Variables|References|SetHUD_Ref (Utilities|Array|Get(acopy) _foundwidgets))
  (return))

(fn SetStunnedVariables
  (if (Variables|Bools|GetIsFirstStun?)
    (Variables|Bools|SetIsFirstStun? false)
    (Default|PauseGameplay (Variables|References|GetPlayer_Ref) false false false true false))
  (Variables|Bools|SetIsStunned? true)
  (Variables|/Game/MyContent/Blueprints/Players/BP_Player.BP_Player_C|SetIsStunned? (Variables|References|GetPlayer_Ref) true)
  (Math|Integer|IncrementInt (Variables|/Game/MyContent/Blueprints/Players/BP_Player.BP_Player_C|GetPedestrianNumberStunned (Variables|References|GetPlayer_Ref))
    (:%20%20
      (return))))

(fn ResetFollowStreet
  (params (IsGameOver? :type Boolean))
  (bind _hud_ref (Variables|References|GetHUD_Ref))
  (bind _player_ref (Variables|References|GetPlayer_Ref))
  (bind _hud_ref_2 (Variables|References|GetHUD_Ref))
  (bind _w_scoreboard_combo (Variables|/Game/MyContent/Blueprints/Widgets/HUD/W_HUD.W_HUD_C|GetW_Scoreboard_Combo _hud_ref_2))
  (if (and (Variables|/Game/MyContent/Blueprints/Players/BP_Player.BP_Player_C|GetIsFirstScore? (Variables|References|GetPlayer_Ref)) (== (Variables|/Game/MyContent/Blueprints/Widgets/HUD/W_Scoreboard_Combo.W_Scoreboard_Combo_C|GetPedestrianCombo (Variables|/Game/MyContent/Blueprints/Widgets/HUD/W_HUD.W_HUD_C|GetW_Scoreboard_Combo (Variables|References|GetHUD_Ref))) 1))
    (Variables|/Game/MyContent/Blueprints/Players/BP_Player.BP_Player_C|SetIsFirstScore? _player_ref false)
    (Default|PauseGameplay _player_ref false false true false false))
  (LocalVariables|SetIsGameOver?_Loc IsGameOver?)
  (Variables|Bools|SetIsComplemented? false)
  (Variables|Bools|SetIsStunned? false)
  (Variables|Bools|SetIsFollowingPlayer? false)
  (bind _result (Math|Integer|DecrementInt (Variables|/Game/MyContent/Blueprints/Widgets/HUD/W_Scoreboard_Combo.W_Scoreboard_Combo_C|GetPedestrianCombo _w_scoreboard_combo))
    (:%20%20
      (bind _output_get (Variables|/Game/MyContent/Blueprints/Widgets/HUD/W_Scoreboard_Combo.W_Scoreboard_Combo_C|SetPedestrianCombo _w_scoreboard_combo _result))
      (if (<= _output_get 0)
        (Widget|SetVisibility (Variables|/Game/MyContent/Blueprints/Widgets/HUD/W_HUD.W_HUD_C|GetW_Scoreboard_Combo (Variables|References|GetHUD_Ref)) "Hidden")
        (Variables|/Game/MyContent/Blueprints/Widgets/HUD/W_Scoreboard_Streak.W_Scoreboard_Streak_C|SetIsIncreasing? (Variables|/Game/MyContent/Blueprints/Widgets/HUD/W_Scoreboard.W_Scoreboard_C|GetW_Scoreboard_Streak (Variables|/Game/MyContent/Blueprints/Widgets/HUD/W_HUD.W_HUD_C|GetW_Scoreboard _hud_ref)) false)
        (if (not (LocalVariables|GetIsGameOver?_Loc))
          (Default|SetScoreValue _hud_ref)))
      (return))))

(fn UpdatePedestrianCombo
  (bind _hud_ref (Variables|References|GetHUD_Ref))
  (bind _w_scoreboard_combo (Variables|/Game/MyContent/Blueprints/Widgets/HUD/W_HUD.W_HUD_C|GetW_Scoreboard_Combo _hud_ref))
  (bind _result (Math|Integer|IncrementInt (Variables|/Game/MyContent/Blueprints/Widgets/HUD/W_Scoreboard_Combo.W_Scoreboard_Combo_C|GetPedestrianCombo _w_scoreboard_combo))
    (:%20%20
      (Variables|/Game/MyContent/Blueprints/Widgets/HUD/W_Scoreboard_Combo.W_Scoreboard_Combo_C|SetPedestrianCombo _w_scoreboard_combo _result)
      (Widget|SetVisibility (Variables|/Game/MyContent/Blueprints/Widgets/HUD/W_HUD.W_HUD_C|GetW_Scoreboard_Combo (Variables|References|GetHUD_Ref)) "Visible")
      (return))))

(fn IncreaseBatteryReduceRate
  (bind _player_ref (Variables|References|GetPlayer_Ref))
  (bind _result (Math|Integer|IncrementInt (Variables|/Game/MyContent/Blueprints/Players/BP_Player.BP_Player_C|GetPedestrianNumberColliding _player_ref))
    (:%20%20
      (bind _output_get (Variables|/Game/MyContent/Blueprints/Players/BP_Player.BP_Player_C|SetPedestrianNumberColliding _player_ref _result))
      (Default|SetFillColourandReduceValue (Variables|/Game/MyContent/Blueprints/Widgets/HUD/W_HUD.W_HUD_C|GetW_Battery (Variables|References|GetHUD_Ref)) _output_get)
      (return))))

(fn DecreaseBatteryReduceRate
  (bind _player_ref (Variables|References|GetPlayer_Ref))
  (bind _result (Math|Integer|DecrementInt (Variables|/Game/MyContent/Blueprints/Players/BP_Player.BP_Player_C|GetPedestrianNumberColliding _player_ref))
    (:%20%20
      (bind _output_get (Variables|/Game/MyContent/Blueprints/Players/BP_Player.BP_Player_C|SetPedestrianNumberColliding _player_ref _result))
      (Default|SetFillColourandReduceValue (Variables|/Game/MyContent/Blueprints/Widgets/HUD/W_HUD.W_HUD_C|GetW_Battery (Variables|References|GetHUD_Ref)) _output_get)
      (return))))

(fn UpdatePedestriansFollowingPlayer
  (params (IsFollowingPlayer? :type Boolean))
  (if IsFollowingPlayer?
    (return)
    (else
      (Utilities|Array|RemoveItem (Variables|/Game/MyContent/Blueprints/Players/BP_Player.BP_Player_C|GetPedestriansFollowingPlayer (Variables|References|GetPlayer_Ref)) self)
      (return))))

(fn DestroySelf
  (bind _gamemode_ref (Variables|References|GetGameMode_Ref))
  (bind _result (Math|Integer|DecrementInt (Variables|/Game/MyContent/Blueprints/GameModes/GM_Infinite.GM_Infinite_C|GetPedestrianNumberSpawned _gamemode_ref))
    (:%20%20
      (Variables|/Game/MyContent/Blueprints/GameModes/GM_Infinite.GM_Infinite_C|SetPedestrianNumberSpawned _gamemode_ref _result)
      (Utilities|Array|RemoveItem (Variables|/Game/MyContent/Blueprints/Players/BP_Player.BP_Player_C|GetPedestrian_Refs (Variables|References|GetPlayer_Ref)) self)
      (if (Utilities|Enum|Equal(Enum) (Utilities|GetDisplayName (Variables|/Game/MyContent/Blueprints/Players/BP_Player.BP_Player_C|GetTargetPedestrian_Ref (Variables|References|GetPlayer_Ref))) (Utilities|GetDisplayName self))
        (Variables|/Game/MyContent/Blueprints/Players/BP_Player.BP_Player_C|SetTargetPedestrian_Ref (Variables|References|GetPlayer_Ref) 0))
      (Actor|DestroyActor)
      (return))))

(fn GetDistancefromPlayer
  (bind _player_ref (Variables|References|GetPlayer_Ref))
  (return (<= (Math|Vector|Distance(Vector) (Transformation|GetActorLocation self) (Transformation|GetActorLocation _player_ref)) (* (Variables|/Game/MyContent/Blueprints/Players/BP_Player.BP_Player_C|GetEscapeRange _player_ref) 1.0))))
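; BP_Player_Tutorial is a tutorial player Blueprint that advances dialogue text in the tutorial HUD.
; Left mouse button or Space increments the dialogue widget's text index and refreshes the shown block.
; Helper functions find BP_Player and W_HUD_Tutorial and possess or unpossess the player pawn.
; BeginPlay is empty and the setup calls are disconnected, so this Blueprint never assigns its HUD reference itself.
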(event EventBeginPlay)

(event Input|KeyboardEvents|SpaceBar
  (params (Key :type Key%20Structure :default "None"))
  (bind _hud_tutorial_ref (Variables|Default|GetHUD_Tutorial_Ref))
  (bind _w_dialogue (Variables|/Game/MyContent/Blueprints/Widgets/Game/W_HUD_Tutorial.W_HUD_Tutorial_C|GetW_Dialogue _hud_tutorial_ref))
  (:Pressed
    (bind _result (Math|Integer|IncrementInt (Variables|/Game/MyContent/Blueprints/Widgets/Game/W_Dialogue.W_Dialogue_C|GetCurrentTextBlockElement _w_dialogue))
      (:%20%20
        (Variables|/Game/MyContent/Blueprints/Widgets/Game/W_Dialogue.W_Dialogue_C|SetCurrentTextBlockElement _w_dialogue _result)
        (Default|SetCurrentTextBlock _w_dialogue)))))

(event Input|MouseEvents|LeftMouseButton
  (params (Key :type Key%20Structure :default "None"))
  (bind _hud_tutorial_ref (Variables|Default|GetHUD_Tutorial_Ref))
  (bind _w_dialogue (Variables|/Game/MyContent/Blueprints/Widgets/Game/W_HUD_Tutorial.W_HUD_Tutorial_C|GetW_Dialogue _hud_tutorial_ref))
  (:Pressed
    (bind _result (Math|Integer|IncrementInt (Variables|/Game/MyContent/Blueprints/Widgets/Game/W_Dialogue.W_Dialogue_C|GetCurrentTextBlockElement _w_dialogue))
      (:%20%20
        (Variables|/Game/MyContent/Blueprints/Widgets/Game/W_Dialogue.W_Dialogue_C|SetCurrentTextBlockElement _w_dialogue _result)
        (Default|SetCurrentTextBlock _w_dialogue)))))

(fn ConstructionScript)

(fn SetReferences
  (bind _outactors (Actor|GetAllActorsOfClass "/Game/MyContent/Blueprints/Players/BP_Player.BP_Player_C"))
  (Variables|Default|SetPlayer_Ref (Utilities|Array|Get(acopy) _outactors))
  (bind _foundwidgets (Widget|GetAllWidgetsOfClass "/Game/MyContent/Blueprints/Widgets/Game/W_HUD_Tutorial.W_HUD_Tutorial_C" true))
  (Variables|Default|SetHUD_Tutorial_Ref (Utilities|Array|Get(acopy) _foundwidgets))
  (return))

(fn PossessPlayer
  (Pawn|Possess (Game|GetPlayerController 0) (Game|Player|GetPlayerPawn 0))
  (Development|PrintString "Hello")
  (return))

(fn UnPossessPlayer
  (Pawn|UnPossess (Game|GetPlayerController 0))
  (return))
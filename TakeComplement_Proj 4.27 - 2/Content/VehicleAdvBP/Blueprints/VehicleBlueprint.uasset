(event EventBeginPlay
  (CallFunction|CreateWidgets)
  (CallFunction|SetCamera))

(event EventTick
  (params (DeltaSeconds :type Float%20%28single-precision%29))
  (CallFunction|UpdatePlayerMovement)
  (if (Variables|Default|GetIsPlaying?)
    (if (Variables|/Game/MyContent/Blueprints/Widgets/Game/W_Battery.W_Battery_C|GetIsBatteryEmpty? (Variables|/Game/MyContent/Blueprints/Widgets/Game/W_HUD.W_HUD_C|GetW_Battery (Variables|Default|GetHUD_Ref)))
      (CallFunction|ThankPlayer)
      (else
        (bind (_returnvalue _hitactor) (CallFunction|CheckActorUnderCrosshair (Variables|Default|GetHUD_Ref)))
        (if (Variables|Default|GetIsCrosshairValid?)
          (CallFunction|IsTargetPedestrianValid _returnvalue _hitactor)
          (CallFunction|SetTargetPedestrian)
          (bind _isvalid_ (CallFunction|IsTargetPedestrianStillActive))
          (CallFunction|UpdateCrosshair _isvalid_)
          (CallFunction|SetPedestrianOutlineColour))))))

(event Input|AxisEvents|InputAxisMoveForward
  (params (AxisValue :type Float%20%28single-precision%29))
  (Class|WheeledVehicleMovementComponent|SetThrottleInput (Variables|Default|GetVehicleMovement) AxisValue))

(event Input|AxisEvents|InputAxisMoveRight
  (params (AxisValue :type Float%20%28single-precision%29))
  (Class|WheeledVehicleMovementComponent|SetSteeringInput (Variables|Default|GetVehicleMovement) AxisValue))

(event Input|MouseEvents|LeftMouseButton
  (params (Key :type Key%20Structure :default "None"))
  (:Pressed
    (if (Utilities|Enum|Equal(Enum) (Utilities|GetDisplayName (Variables|Default|GetTargetPedestrian_Ref)) "")
      (Variables|Default|SetIsPedestrianHighlighted? false)
      (elif (UserInterface|Viewport|IsinViewport (Variables|/Game/MyContent/Blueprints/Widgets/Game/W_HUD.W_HUD_C|GetW_Crosshair (Variables|Default|GetHUD_Ref)))
        (if (not (Variables|/Game/MyContent/Blueprints/Characters/BP_Pedestrian.BP_Pedestrian_C|GetIsTooClose? (Variables|Default|GetTargetPedestrian_Ref)))
          (Variables|Default|SetIsPedestrianHighlighted? true)
          (if (not (Variables|/Game/MyContent/Blueprints/Characters/BP_Pedestrian.BP_Pedestrian_C|GetIsCollidingWithPlayer? (Variables|Default|GetTargetPedestrian_Ref)))
            (CallFunction|SetPedestriantoFollowPlayer)
            (Rendering|SetCustomDepthStencilValue (Variables|/Script/Engine.Character|GetMesh (Variables|Default|GetTargetPedestrian_Ref)) 3)
            (if (Variables|Default|GetIsPedestrianHighlighted?)
              (CallFunction|UpdatePlayerBattery)
              (CallFunction|UpdatePlayerScoreCombo)
              (CallFunction|UpdatePlayerScoreStreak))
            (else
              (CallFunction|IncreaseMovementSpeed)))
          (else
            (Variables|Default|SetIsPedestrianHighlighted? false :!label _label)))
        (else
          (goto _label))))))

(fn ConstructionScript)

(fn CreateWidgets
  (bind _returnvalue (UserInterface|CreateWidget "/Game/MyContent/Blueprints/Widgets/Game/W_HUD.W_HUD_C"))
  (bind _output_get (Variables|Default|SetHUD_Ref _returnvalue))
  (UserInterface|Viewport|AddtoViewport _output_get 0)
  (return))

(fn SetCamera
  (if (Variables|Default|GetIsPlaying?)
    (Components|Activation|Activate (Variables|Camera|GetCamera) false)
    (return)))

(fn CheckActorUnderCrosshair
  (params (HUD_Ref :type W%20HUD%20Object%20Reference))
  (bind _camera (Variables|Camera|GetCamera))
  (bind _returnvalue (Transformation|GetWorldLocation _camera))
  (Variables|/Game/MyContent/Blueprints/Widgets/Game/W_HUD.W_HUD_C|GetW_Crosshair HUD_Ref
    (:then
      (Variables|Default|SetIsCrosshairValid? true)
      (bind (_outhit _returnvalue_2) (Collision|LineTraceByChannel _returnvalue (+ _returnvalue (* (Math|Vector|GetForwardVector _camera) (Variables|Default|GetComplementRange))) "TraceTypeQuery2" false 0 "None")))
    (:else
      (Variables|Default|SetIsCrosshairValid? false)))
  (return _returnvalue_2 (.HitActor (Collision|BreakHitResult _outhit))))

(fn SetTargetPedestrian
  (if (Variables|Default|GetIsInRange?)
    (bind _array_element (Utilities|Array|ForEachLoopwithBreak (Variables|Default|GetPedestrian_Refs) :!label _label)
      (:LoopBody
        (if (Utilities|Name|Equal(Name) (Utilities|Array|Get(acopy) (Variables|/Script/Engine.Actor|GetTags _array_element)) (Variables|Default|GetPedestrianID_Ref))
          (bind _output_get (Variables|Default|SetTargetPedestrian_Ref _array_element))
          (Variables|/Game/MyContent/Blueprints/Characters/BP_Pedestrian.BP_Pedestrian_C|SetIsTargeted? _output_get true)
          (goto _label Break)
          (else
            (Variables|Default|SetTargetPedestrian_Ref 0)
            (Variables|/Game/MyContent/Blueprints/Characters/BP_Pedestrian.BP_Pedestrian_C|SetIsTargeted? _array_element false))))
      (:Completed
        (return)))
    (else
      (return))))

(fn SetPedestriantoFollowPlayer
  (bind _targetpedestrian_ref (Variables|Default|GetTargetPedestrian_Ref))
  (if (Variables|/Game/MyContent/Blueprints/Characters/BP_Pedestrian.BP_Pedestrian_C|GetIsFollowingPlayer? _targetpedestrian_ref)
    _
    (else
      (Variables|/Game/MyContent/Blueprints/Characters/BP_Pedestrian.BP_Pedestrian_C|SetIsFollowingPlayer? _targetpedestrian_ref true)))
  (return))

(fn ThankPlayer
  (return))

(fn UpdatePlayerBattery
  (bind _targetpedestrian_ref (Variables|Default|GetTargetPedestrian_Ref))
  (if (Variables|/Game/MyContent/Blueprints/Characters/BP_Pedestrian.BP_Pedestrian_C|GetIsFollowingPlayer? _targetpedestrian_ref)
    (if (Variables|/Game/MyContent/Blueprints/Characters/BP_Pedestrian.BP_Pedestrian_C|GetIsComplemented? _targetpedestrian_ref)
      _
      (else
        (Default|IncreaseBatteryPercentage (Variables|/Game/MyContent/Blueprints/Widgets/Game/W_HUD.W_HUD_C|GetW_Battery (Variables|Default|GetHUD_Ref)))
        (Variables|/Game/MyContent/Blueprints/Characters/BP_Pedestrian.BP_Pedestrian_C|SetIsComplemented? (Variables|Default|GetTargetPedestrian_Ref) true))))
  (return))

(fn UpdatePlayerMovement
  (bind _camera (Variables|Camera|GetCamera))
  (bind _relativerotation (Variables|/Script/Engine.SceneComponent|GetRelativeRotation _camera))
  (bind (_roll _pitch _yaw) (Math|Rotator|BreakRotator _relativerotation))
  (Variables|Game|SetInReverseGear (< (Class|WheeledVehicleMovementComponent|GetCurrentGear (Variables|Default|GetVehicleMovement)) 0))
  (if (Variables|Default|GetIsPlaying?)
    (Transformation|SetRelativeRotation (Variables|Camera|GetCamera) (Math|Rotator|MakeRotator 0.0 (Math|Float|ClampAngle (+ (Input|AxisValues|GetLookUp) _pitch) -9e+01 9e+01) (+ (Input|AxisValues|GetLookRight) _yaw)) false false)))

(fn UpdatePlayerScore)

(fn UpdatePlayerScoreCombo
  (if (Variables|/Game/MyContent/Blueprints/Characters/BP_Pedestrian.BP_Pedestrian_C|GetIsAddedToScoreCombo? (Variables|Default|GetTargetPedestrian_Ref))
    _
    (else
      (Math|Integer|IncrementInt (Variables|/Game/MyContent/Blueprints/Widgets/Game/W_ScoreCombo.W_ScoreCombo_C|GetScoreCombo (Variables|/Game/MyContent/Blueprints/Widgets/Game/W_HUD.W_HUD_C|GetW_ScoreCombo (Variables|Default|GetHUD_Ref)))
        (:%20%20
          (Variables|/Game/MyContent/Blueprints/Characters/BP_Pedestrian.BP_Pedestrian_C|SetIsAddedToScoreCombo? (Variables|Default|GetTargetPedestrian_Ref) true)))))
  (return))

(fn UpdatePlayerScoreStreak
  (if (Variables|/Game/MyContent/Blueprints/Widgets/Game/W_ScoreStreak.W_ScoreStreak_C|GetIsIncreasing? (Variables|/Game/MyContent/Blueprints/Widgets/Game/W_HUD.W_HUD_C|GetW_ScoreStreak (Variables|Default|GetHUD_Ref)))
    _
    (else
      (Variables|/Game/MyContent/Blueprints/Widgets/Game/W_ScoreStreak.W_ScoreStreak_C|SetIsIncreasing? (Variables|/Game/MyContent/Blueprints/Widgets/Game/W_HUD.W_HUD_C|GetW_ScoreStreak (Variables|Default|GetHUD_Ref)) true)))
  (return))

(fn IsTargetPedestrianValid
  (params (ReturnValue :type Boolean) (HitActor :type Actor%20Object%20Reference))
  (bind _returnvalue (Utilities|DoesObjectImplementInterface HitActor "/Game/MyContent/Blueprints/Interfaces/BP_ComplementInterface.BP_ComplementInterface_C"))
  (if ReturnValue
    (if (and (not (CallFunction|CheckIsCrosshairActive)) _returnvalue)
      (Variables|Default|SetPedestrianID_Ref (Utilities|Array|Get(acopy) (Variables|/Script/Engine.Actor|GetTags HitActor)))
      (Variables|Default|SetIsInRange? true)
      (else
        (if _returnvalue :!label _label
          _
          (else
            (Variables|Default|SetPedestrianID_Ref "None")
            (Variables|Default|SetIsInRange? false)))))
    (else
      (goto _label)))
  (return))

(fn IsTargetPedestrianStillActive
  (if (Utilities|Enum|Equal(Enum) (Utilities|GetDisplayName (Variables|Default|GetTargetPedestrian_Ref)) "")
    (Variables|Default|SetTargetPedestrian_Ref 0)
    (return false)
    (else
      (return true))))

(fn CheckIsCrosshairActive
  (if (UserInterface|Viewport|IsinViewport (Variables|/Game/MyContent/Blueprints/Widgets/Game/W_HUD.W_HUD_C|GetW_Crosshair (Variables|Default|GetHUD_Ref)))
    (return true)
    (else
      (return false))))

(fn UpdateCrosshair
  (params (IsValid? :type Boolean))
  (if IsValid?
    (if (not (Utilities|Name|Equal(Name) (Variables|Default|GetPedestrianID_Ref) "None"))
      (if (Variables|/Game/MyContent/Blueprints/Characters/BP_Pedestrian.BP_Pedestrian_C|GetIsTooClose? (Variables|Default|GetTargetPedestrian_Ref))
        (if (CallFunction|CheckIsCrosshairActive)
          _
          (else
            (UserInterface|Viewport|AddtoViewport (Variables|/Game/MyContent/Blueprints/Widgets/Game/W_HUD.W_HUD_C|GetW_Crosshair (Variables|Default|GetHUD_Ref)) 0)))
        (Default|SetTooClose (Variables|/Game/MyContent/Blueprints/Widgets/Game/W_HUD.W_HUD_C|GetW_ComplementPrompt (Variables|Default|GetHUD_Ref)))
        (Variables|Default|SetOutlineStencilValue 2)
        (else
          (if (CallFunction|CheckIsCrosshairActive)
            _
            (else
              (UserInterface|Viewport|AddtoViewport (Variables|/Game/MyContent/Blueprints/Widgets/Game/W_HUD.W_HUD_C|GetW_Crosshair (Variables|Default|GetHUD_Ref)) 0)))
          (Default|SetinRange (Variables|/Game/MyContent/Blueprints/Widgets/Game/W_HUD.W_HUD_C|GetW_ComplementPrompt (Variables|Default|GetHUD_Ref)))
          (Variables|Default|SetOutlineStencilValue 1)))
      (if (Variables|/Game/MyContent/Blueprints/Characters/BP_Pedestrian.BP_Pedestrian_C|GetIsCollidingWithPlayer? (Variables|Default|GetTargetPedestrian_Ref))
        (Default|SetCollidedwith (Variables|/Game/MyContent/Blueprints/Widgets/Game/W_HUD.W_HUD_C|GetW_ComplementPrompt (Variables|Default|GetHUD_Ref)))
        (elif (Variables|/Game/MyContent/Blueprints/Characters/BP_Pedestrian.BP_Pedestrian_C|GetIsFollowingPlayer? (Variables|Default|GetTargetPedestrian_Ref))
          (Default|SetFollowing (Variables|/Game/MyContent/Blueprints/Widgets/Game/W_HUD.W_HUD_C|GetW_ComplementPrompt (Variables|Default|GetHUD_Ref)))))
      (else
        (if (CallFunction|CheckIsCrosshairActive) :!label _label
          (Widget|RemovefromParent (Variables|/Game/MyContent/Blueprints/Widgets/Game/W_HUD.W_HUD_C|GetW_Crosshair (Variables|Default|GetHUD_Ref))))
        (Default|SetOutOfRange (Variables|/Game/MyContent/Blueprints/Widgets/Game/W_HUD.W_HUD_C|GetW_ComplementPrompt (Variables|Default|GetHUD_Ref)))
        (Variables|Default|SetOutlineStencilValue 0)))
    (else
      (goto _label)))
  (return))

(fn SetPedestrianOutlineColour
  (bind _targetpedestrian_ref (Variables|Default|GetTargetPedestrian_Ref))
  (if (CallFunction|CheckIsCrosshairActive)
    (Rendering|SetCustomDepthStencilValue (Variables|/Script/Engine.Character|GetMesh _targetpedestrian_ref) (Variables|Default|GetOutlineStencilValue) :!label _label)
    (if (Variables|/Game/MyContent/Blueprints/Characters/BP_Pedestrian.BP_Pedestrian_C|GetIsCollidingWithPlayer? _targetpedestrian_ref)
      (bind _output_get (Variables|Default|SetOutlineStencilValue 4))
      (Rendering|SetCustomDepthStencilValue (Variables|/Script/Engine.Character|GetMesh (Variables|Default|GetTargetPedestrian_Ref)) _output_get))
    (elif (not (Utilities|Enum|Equal(Enum) (Utilities|GetDisplayName (Variables|Default|GetTargetPedestrian_Ref)) ""))
      (if (< (Variables|Default|GetOutlineStencilValue) 2)
        (goto _label)
        (else
          _))))
  (return))

(fn DecreaseMovementSpeed
  (CallFunction|SetPedestrianOutlineColour)
  (return))

(fn IncreaseMovementSpeed
  (Variables|/Game/MyContent/Blueprints/Characters/BP_Pedestrian.BP_Pedestrian_C|SetIsCollidingWithPlayer? (Variables|Default|GetTargetPedestrian_Ref) false)
  (return))
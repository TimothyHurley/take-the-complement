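; Player vehicle pawn that compliments pedestrians so they follow it, charging the HUD battery, or apologises to stunned ones.
; Each tick a camera line trace finds a pedestrian by interface and tag, driving crosshair, name prompts, custom-depth stencil outline and follower range meter.
; Left click acts on the target with random comment popups, while stun reduces throttle per stunned pedestrian.
; StopGameplay runs on empty battery, but its game-over logic is disconnected.
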(event EventBeginPlay
  (CallFunction|StartGameplay))

(event EventTick
  (params (DeltaSeconds :type Float%20%28single-precision%29))
  (if (Variables|Bools|GetIsPlaying?)
    (CallFunction|SetPlayerPositionandRotation)
    (if (Variables|/Game/MyContent/Blueprints/Widgets/HUD/W_Battery.W_Battery_C|GetIsEmpty? (Variables|/Game/MyContent/Blueprints/Widgets/HUD/W_HUD.W_HUD_C|GetW_Battery (Variables|References|GetHUD_Ref)))
      (CallFunction|StopGameplay)
      (else
        (bind (_returnvalue _hitactor) (CallFunction|GetTargetActor (Variables|References|GetHUD_Ref)))
        (if (Variables|Bools|GetIsCrosshairValid?)
          (CallFunction|IdentifyTargetActor _returnvalue _hitactor)
          (CallFunction|SetTargetPedestrian)
          (CallFunction|SetTargetPedestrianState)
          (CallFunction|SetCrosshairState (CallFunction|GetTargetPedestrianValidity))
          (CallFunction|SetTargetPedestrianOutline)
          (if (> (Utilities|Array|Length (Variables|References|GetPedestriansFollowingPlayer)) 0)
            (CallFunction|SetRangeMeterPercent)))))))

(event Input|AxisEvents|InputAxisMoveForward
  (params (AxisValue :type Float%20%28single-precision%29))
  (if (Variables|Bools|GetIsStunned?)
    (Class|WheeledVehicleMovementComponent|SetThrottleInput (Variables|Default|GetVehicleMovement) (/ (* (Variables|Default|GetMovementSpeedMultiplier) AxisValue) (+ (* (Variables|Default|GetPedestrianNumberStunned) (Variables|Default|GetMovementSpeedDivisor)) 1.0)))
    (else
      (Class|WheeledVehicleMovementComponent|SetThrottleInput (Variables|Default|GetVehicleMovement) (* (Variables|Default|GetMovementSpeedMultiplier) AxisValue)))))

(event Input|AxisEvents|InputAxisMoveRight
  (params (AxisValue :type Float%20%28single-precision%29))
  (Class|WheeledVehicleMovementComponent|SetSteeringInput (Variables|Default|GetVehicleMovement) AxisValue))

(event Input|MouseEvents|LeftMouseButton
  (params (Key :type Key%20Structure))
  (bind _targetpedestrian_ref (Variables|References|GetTargetPedestrian_Ref))
  (:Pressed
    (if (and (CallFunction|GetTargetPedestrianValidity) (CallFunction|GetCrosshairValidity))
      (if (Variables|/Game/MyContent/Blueprints/Characters/BP_Pedestrian.BP_Pedestrian_C|GetIsStunned? (Variables|References|GetTargetPedestrian_Ref))
        (CallFunction|ApologisetoPedestrian)
        (CallFunction|UpdateRecipientApology false)
        (CallFunction|UpdateCommentApology true)
        (Utilities|FlowControl|Delay 2.0)
        (CallFunction|UpdateCommentApology false)
        (elif (not (Variables|/Game/MyContent/Blueprints/Characters/BP_Pedestrian.BP_Pedestrian_C|GetIsFollowingPlayer? (Variables|References|GetTargetPedestrian_Ref)))
          (Variables|/Game/MyContent/Blueprints/Characters/BP_Pedestrian.BP_Pedestrian_C|SetIsFollowingPlayer? _targetpedestrian_ref true)
          (Utilities|Array|Add (Variables|References|GetPedestriansFollowingPlayer) _targetpedestrian_ref)
          (CallFunction|SetBatteryPercent)
          (CallFunction|UpdateScoreStreak)
          (CallFunction|UpdateCommentComplement true)
          (Utilities|FlowControl|Delay 2.0)
          (CallFunction|UpdateCommentComplement false))))))

(fn ConstructionScript)

(fn StartGameplay
  (bind _returnvalue (UserInterface|CreateWidget "/Game/MyContent/Blueprints/Widgets/HUD/W_HUD.W_HUD_C"))
  (bind _output_get (Variables|References|SetHUD_Ref _returnvalue))
  (UserInterface|Viewport|AddtoViewport _output_get 0)
  (Variables|/Script/Engine.PlayerController|SetbShowMouseCursor (Game|GetPlayerController 0) false)
  (Variables|Bools|SetIsPlaying? true)
  (return))

(fn StopGameplay)

(fn SetPlayerPositionandRotation
  (bind _camera (Variables|Components|GetCamera))
  (bind _relativerotation (Variables|/Script/Engine.SceneComponent|GetRelativeRotation _camera))
  (bind (_roll _pitch _yaw) (Math|Rotator|BreakRotator _relativerotation))
  (Variables|Bools|SetIsReversing? (< (Class|WheeledVehicleMovementComponent|GetCurrentGear (Variables|Default|GetVehicleMovement)) 0))
  (Transformation|SetRelativeRotation (Variables|Components|GetCamera) (Math|Rotator|MakeRotator 0.0 (Math|Float|ClampAngle (+ (Input|AxisValues|GetLookUp) _pitch) -9e+01 9e+01) (+ (Input|AxisValues|GetLookRight) _yaw)) false false)
  (return))

(fn SetCrosshairState
  (params (IsValid? :type Boolean))
  (if IsValid?
    (if (not (Utilities|Name|Equal(Name) (Variables|References|GetPedestrianID_Ref) "None"))
      (if (CallFunction|GetCrosshairValidity)
        _
        (else
          (UserInterface|Viewport|AddtoViewport (Variables|/Game/MyContent/Blueprints/Widgets/HUD/W_HUD.W_HUD_C|GetW_Crosshair (Variables|References|GetHUD_Ref)) 0)))
      (else
        (if (CallFunction|GetCrosshairValidity) :!label _label
          (Widget|RemovefromParent (Variables|/Game/MyContent/Blueprints/Widgets/HUD/W_HUD.W_HUD_C|GetW_Crosshair (Variables|References|GetHUD_Ref))))))
    (else
      (goto _label)))
  (return))

(fn SetTargetPedestrian
  (for _array_element (Variables|References|GetPedestrian_Refs)
    (Variables|/Game/MyContent/Blueprints/Characters/BP_Pedestrian.BP_Pedestrian_C|SetIsReferenced? _array_element false))
  (if (Variables|Bools|GetIsInRange?)
    (bind _array_element_2 (Utilities|Array|ForEachLoopwithBreak (Variables|References|GetPedestrian_Refs) :!label _label)
      (:LoopBody
        (if (Utilities|Name|Equal(Name) (Utilities|Array|Get(acopy) (Variables|/Script/Engine.Actor|GetTags _array_element_2)) (Variables|References|GetPedestrianID_Ref))
          (bind _output_get (Variables|References|SetTargetPedestrian_Ref _array_element_2))
          (Variables|/Game/MyContent/Blueprints/Characters/BP_Pedestrian.BP_Pedestrian_C|SetIsReferenced? _output_get true)
          (goto _label Break)
          (else
            (Variables|References|SetTargetPedestrian_Ref 0)
            (Variables|/Game/MyContent/Blueprints/Characters/BP_Pedestrian.BP_Pedestrian_C|SetIsReferenced? _array_element_2 false))))
      (:Completed
        (return)))
    (else
      (return))))

(fn SetTargetPedestrianState
  (bind _targetpedestrian_ref (Variables|References|GetTargetPedestrian_Ref))
  (if (CallFunction|GetTargetPedestrianValidity)
    (if (Variables|/Game/MyContent/Blueprints/Characters/BP_Pedestrian.BP_Pedestrian_C|GetIsStunned? (Variables|References|GetTargetPedestrian_Ref))
      (Variables|Default|SetOutlineStencilValue 4)
      (if (CallFunction|GetCrosshairValidity)
        (CallFunction|UpdateRecipientApology true)
        (else
          (CallFunction|UpdateRecipientApology false)
          (if (CallFunction|GetCrosshairValidity) :!label _label
            (CallFunction|UpdateRecipientComplement true)
            (else
              (CallFunction|UpdateRecipientComplement false)))))
      (elif (Variables|/Game/MyContent/Blueprints/Characters/BP_Pedestrian.BP_Pedestrian_C|GetIsFollowingPlayer? (Variables|References|GetTargetPedestrian_Ref))
        (Variables|Default|SetOutlineStencilValue 3)
        (goto _label)
        (elif (CallFunction|GetCrosshairValidity)
          (Variables|Default|SetOutlineStencilValue 1)
          (CallFunction|UpdateRecipientComplement true)
          (else
            (if (not (and (Variables|/Game/MyContent/Blueprints/Characters/BP_Pedestrian.BP_Pedestrian_C|GetIsStunned? _targetpedestrian_ref) (Variables|/Game/MyContent/Blueprints/Characters/BP_Pedestrian.BP_Pedestrian_C|GetIsFollowingPlayer? _targetpedestrian_ref)))
              (Variables|Default|SetOutlineStencilValue 0))
            (CallFunction|UpdateRecipientComplement false))))))
  (return))

(fn SetTargetPedestrianOutline
  (bind _targetpedestrian_ref (Variables|References|GetTargetPedestrian_Ref))
  (bind _targetpedestrian_ref_2 (Variables|References|GetTargetPedestrian_Ref))
  (if (CallFunction|GetCrosshairValidity)
    (Rendering|SetCustomDepthStencilValue (Variables|/Script/Engine.Character|GetMesh _targetpedestrian_ref_2) (Variables|Default|GetOutlineStencilValue) :!label _label)
    (if (Variables|/Game/MyContent/Blueprints/Characters/BP_Pedestrian.BP_Pedestrian_C|GetIsStunned? _targetpedestrian_ref_2)
      (bind _output_get (Variables|Default|SetOutlineStencilValue 4))
      (Rendering|SetCustomDepthStencilValue (Variables|/Script/Engine.Character|GetMesh _targetpedestrian_ref) _output_get)
      (Components|Movement|StopMovementImmediately (Variables|/Script/Engine.Character|GetCharacterMovement _targetpedestrian_ref)))
    (elif (not (Utilities|Enum|Equal(Enum) (Utilities|GetDisplayName (Variables|References|GetTargetPedestrian_Ref)) ""))
      (if (< (Variables|Default|GetOutlineStencilValue) 2)
        (goto _label)
        (else
          _))))
  (return))

(fn SetBatteryPercent
  (bind _targetpedestrian_ref (Variables|References|GetTargetPedestrian_Ref))
  (if (and (Variables|/Game/MyContent/Blueprints/Characters/BP_Pedestrian.BP_Pedestrian_C|GetIsFollowingPlayer? _targetpedestrian_ref) (not (Variables|/Game/MyContent/Blueprints/Characters/BP_Pedestrian.BP_Pedestrian_C|GetIsComplemented? _targetpedestrian_ref)))
    (Default|IncreaseBatteryPercent (Variables|/Game/MyContent/Blueprints/Widgets/HUD/W_HUD.W_HUD_C|GetW_Battery (Variables|References|GetHUD_Ref)))
    (Variables|/Game/MyContent/Blueprints/Characters/BP_Pedestrian.BP_Pedestrian_C|SetIsComplemented? (Variables|References|GetTargetPedestrian_Ref) true))
  (return))

(fn SetRangeMeterPercent
  (for _array_element (Variables|References|GetPedestriansFollowingPlayer)
    (if (> (LocalVariables|GetPercent_Loc) (Math|Float|SafeDivide (Math|Float|Absolute(Float) (Math|Vector|Distance(Vector) (Transformation|GetActorLocation) (Transformation|GetActorLocation _array_element))) (Variables|Default|GetEscapeRange)))
      (LocalVariables|SetPercent_Loc (Math|Float|SafeDivide (Math|Float|Absolute(Float) (Math|Vector|Distance(Vector) (Transformation|GetActorLocation) (Transformation|GetActorLocation _array_element))) (Variables|Default|GetEscapeRange)))))
  (Progress|SetPercent (Variables|/Game/MyContent/Blueprints/Widgets/HUD/W_RangeMeter.W_RangeMeter_C|GetRangeMeter_ProgressBar (Variables|/Game/MyContent/Blueprints/Widgets/HUD/W_HUD.W_HUD_C|GetW_RangeMeter (Variables|References|GetHUD_Ref))) (LocalVariables|GetPercent_Loc))
  (return))

(fn GetTargetActor
  (params (HUD_Ref :type W%20HUD%20Object%20Reference))
  (bind _camera (Variables|Components|GetCamera))
  (bind _returnvalue (Transformation|GetWorldLocation _camera))
  (Variables|/Game/MyContent/Blueprints/Widgets/HUD/W_HUD.W_HUD_C|GetW_Crosshair HUD_Ref
    (:then
      (Variables|Bools|SetIsCrosshairValid? true)
      (bind (_outhit _returnvalue_2) (Collision|LineTraceByChannel _returnvalue (+ _returnvalue (* (Math|Vector|GetForwardVector _camera) (Variables|Default|GetComplementRange))) "TraceTypeQuery2" false 0 "None"))
      (return _returnvalue_2 (.HitActor (Collision|BreakHitResult _outhit))))
    (:else
      (Variables|Bools|SetIsCrosshairValid? false)
      (return false 0))))

(fn IdentifyTargetActor
  (params (ReturnValue :type Boolean) (HitActor :type Actor%20Object%20Reference))
  (if ReturnValue
    (if (Utilities|DoesObjectImplementInterface HitActor "/Game/MyContent/Blueprints/Interfaces/BP_ComplementInterface.BP_ComplementInterface_C")
      (Variables|References|SetPedestrianID_Ref (Utilities|Array|Get(acopy) (Variables|/Script/Engine.Actor|GetTags HitActor)))
      (Variables|Bools|SetIsInRange? true)
      (else
        (Variables|References|SetPedestrianID_Ref "" :!label _label)
        (Variables|Bools|SetIsInRange? false)))
    (else
      (goto _label)))
  (return))

(fn ApologisetoPedestrian
  (Utilities|FlowControl|DoOnce false
    (:Completed
      (bind _result (Math|Integer|DecrementInt (Variables|Default|GetPedestrianNumberStunned))
        (:%20%20
          (if (<= _result 0)
            (Variables|Default|SetPedestrianNumberStunned 0)
            (Variables|Bools|SetIsStunned? false))
          (Default|AnimateCornersReverse (Variables|References|GetHUD_Ref) (Variables|Default|GetPedestrianNumberStunned))
          (Variables|/Game/MyContent/Blueprints/Characters/BP_Pedestrian.BP_Pedestrian_C|SetIsStunned? (Variables|References|GetTargetPedestrian_Ref) false)
          (return))))))

(fn UpdateRecipientApology
  (params (IsVisible? :type Boolean))
  (bind _hud_ref (Variables|References|GetHUD_Ref))
  (bind _w_recipient_apology (Variables|/Game/MyContent/Blueprints/Widgets/HUD/W_HUD.W_HUD_C|GetW_Recipient_Apology _hud_ref))
  (if IsVisible?
    (UserInterface|Viewport|AddtoViewport _w_recipient_apology 0)
    (Class|UserWidget|SetPositioninViewport :self _w_recipient_apology :bRemoveDPIScale false)
    (Rendering|Components|TextRender|SetText (Variables|/Game/MyContent/Blueprints/Widgets/HUD/W_Recipient_Apology.W_Recipient_Apology_C|GetTextBlock_Name (Variables|/Game/MyContent/Blueprints/Widgets/HUD/W_HUD.W_HUD_C|GetW_Recipient_Apology (Variables|References|GetHUD_Ref))) (Variables|/Game/MyContent/Blueprints/Characters/BP_Pedestrian.BP_Pedestrian_C|GetFullName (Variables|References|GetTargetPedestrian_Ref)))
    (return)
    (else
      (Widget|RemovefromParent (Variables|/Game/MyContent/Blueprints/Widgets/HUD/W_HUD.W_HUD_C|GetW_Recipient_Apology (Variables|References|GetHUD_Ref)))
      (return))))

(fn UpdateRecipientComplement
  (params (IsVisible? :type Boolean))
  (bind _hud_ref (Variables|References|GetHUD_Ref))
  (bind _w_recipient_complement (Variables|/Game/MyContent/Blueprints/Widgets/HUD/W_HUD.W_HUD_C|GetW_Recipient_Complement _hud_ref))
  (if IsVisible?
    (UserInterface|Viewport|AddtoViewport _w_recipient_complement 0)
    (Class|UserWidget|SetPositioninViewport :self _w_recipient_complement :bRemoveDPIScale false)
    (Rendering|Components|TextRender|SetText (Variables|/Game/MyContent/Blueprints/Widgets/HUD/W_Recipient_Complement.W_Recipient_Complement_C|GetTextBlock_Name (Variables|/Game/MyContent/Blueprints/Widgets/HUD/W_HUD.W_HUD_C|GetW_Recipient_Complement (Variables|References|GetHUD_Ref))) (Variables|/Game/MyContent/Blueprints/Characters/BP_Pedestrian.BP_Pedestrian_C|GetFullName (Variables|References|GetTargetPedestrian_Ref)))
    (return)
    (else
      (Widget|RemovefromParent (Variables|/Game/MyContent/Blueprints/Widgets/HUD/W_HUD.W_HUD_C|GetW_Recipient_Complement (Variables|References|GetHUD_Ref)))
      (return))))

(fn UpdateCommentApology
  (params (IsVisible? :type Boolean))
  (bind _hud_ref (Variables|References|GetHUD_Ref))
  (bind _w_comment_apology (Variables|/Game/MyContent/Blueprints/Widgets/HUD/W_HUD.W_HUD_C|GetW_Comment_Apology _hud_ref))
  (if IsVisible?
    (UserInterface|Viewport|AddtoViewport _w_comment_apology 0)
    (Class|UserWidget|SetPositioninViewport _w_comment_apology "(X=651.500000,Y=193.500000)" false)
    (Rendering|Components|TextRender|SetText (Variables|/Game/MyContent/Blueprints/Widgets/HUD/W_Comment_Apology.W_Comment_Apology_C|GetTextBlock_Comment (Variables|/Game/MyContent/Blueprints/Widgets/HUD/W_HUD.W_HUD_C|GetW_Comment_Apology (Variables|References|GetHUD_Ref))) (CallFunction|GetRandomTextfromArray (Variables|Default|GetCommentApologies)))
    (bind _result (Math|Integer|IncrementInt (Variables|Default|GetCommentNumberVisible))
      (:%20%20
        (Variables|Default|SetCommentNumberVisible _result)
        (return)))
    (else
      (Widget|RemovefromParent (Variables|/Game/MyContent/Blueprints/Widgets/HUD/W_HUD.W_HUD_C|GetW_Comment_Apology (Variables|References|GetHUD_Ref)))
      (bind _result_2 (Math|Integer|DecrementInt (Variables|Default|GetCommentNumberVisible))
        (:%20%20
          (Variables|Default|SetCommentNumberVisible _result_2)
          (return))))))

(fn UpdateCommentComplement
  (params (IsVisible? :type Boolean))
  (bind _hud_ref (Variables|References|GetHUD_Ref))
  (bind _w_comment_complement (Variables|/Game/MyContent/Blueprints/Widgets/HUD/W_HUD.W_HUD_C|GetW_Comment_Complement _hud_ref))
  (if IsVisible?
    (UserInterface|Viewport|AddtoViewport _w_comment_complement 0)
    (Class|UserWidget|SetPositioninViewport _w_comment_complement "(X=651.500000,Y=193.500000)" false)
    (Rendering|Components|TextRender|SetText (Variables|/Game/MyContent/Blueprints/Widgets/HUD/W_Comment_Complement.W_Comment_Complement_C|GetTextBlock_Comment (Variables|/Game/MyContent/Blueprints/Widgets/HUD/W_HUD.W_HUD_C|GetW_Comment_Complement (Variables|References|GetHUD_Ref))) (CallFunction|GetRandomTextfromArray (Variables|Default|GetCommentComplements)))
    (bind _result (Math|Integer|IncrementInt (Variables|Default|GetCommentNumberVisible))
      (:%20%20
        (Variables|Default|SetCommentNumberVisible _result)
        (return)))
    (else
      (Widget|RemovefromParent (Variables|/Game/MyContent/Blueprints/Widgets/HUD/W_HUD.W_HUD_C|GetW_Comment_Complement (Variables|References|GetHUD_Ref)))
      (bind _result_2 (Math|Integer|DecrementInt (Variables|Default|GetCommentNumberVisible))
        (:%20%20
          (Variables|Default|SetCommentNumberVisible _result_2)
          (return))))))

(fn UpdateCommentPositions
  (bind _foundwidgets (Widget|GetAllWidgetsOfClass "/Game/MyContent/Blueprints/Widgets/HUD/W_Comment_Apology.W_Comment_Apology_C" true))
  (for _array_element _foundwidgets
    _))

(fn UpdateScoreStreak
  (bind _hud_ref (Variables|References|GetHUD_Ref))
  (bind _w_scoreboard (Variables|/Game/MyContent/Blueprints/Widgets/HUD/W_HUD.W_HUD_C|GetW_Scoreboard _hud_ref))
  (bind _w_scoreboard_streak (Variables|/Game/MyContent/Blueprints/Widgets/HUD/W_Scoreboard.W_Scoreboard_C|GetW_Scoreboard_Streak _w_scoreboard))
  (if (Variables|/Game/MyContent/Blueprints/Widgets/HUD/W_Scoreboard_Streak.W_Scoreboard_Streak_C|GetIsIncreasing? (Variables|/Game/MyContent/Blueprints/Widgets/HUD/W_Scoreboard.W_Scoreboard_C|GetW_Scoreboard_Streak (Variables|/Game/MyContent/Blueprints/Widgets/HUD/W_HUD.W_HUD_C|GetW_Scoreboard (Variables|References|GetHUD_Ref))))
    _
    (else
      (Variables|/Game/MyContent/Blueprints/Widgets/HUD/W_Scoreboard_Streak.W_Scoreboard_Streak_C|SetIsIncreasing? _w_scoreboard_streak true)
      (Widget|SetVisibility _w_scoreboard_streak "Visible")))
  (return))

(fn GetCrosshairValidity
  (if (UserInterface|Viewport|IsinViewport (Variables|/Game/MyContent/Blueprints/Widgets/HUD/W_HUD.W_HUD_C|GetW_Crosshair (Variables|References|GetHUD_Ref)))
    (return true)
    (else
      (return false))))

(fn GetTargetPedestrianValidity
  (if (Utilities|Enum|Equal(Enum) (Utilities|GetDisplayName (Variables|References|GetTargetPedestrian_Ref)) "")
    (Variables|References|SetTargetPedestrian_Ref 0)
    (return false)
    (else
      (return true))))

(fn GetRandomTextfromArray
  (params (TextArray :type Array%20of%20Texts))
  (return (Utilities|Array|Get(acopy) TextArray (Math|Random|RandomInteger (Utilities|Array|Length TextArray)))))
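; Game mode for an infinite mode that populates a street with pedestrians and advances a game stage over time.
; BeginPlay caches the player vehicle and two spawn points, then loops spawning tagged pedestrians at random street-width offsets at either point, targeting the opposite end and registering each with the player.
; Tick increments the stage when rounded game time matches the current stage threshold, counting time only in the target level.
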(event EventBeginPlay
  (CallFunction|SetReferencesandSpawnLocations)
  (CallFunction|SpawnPedestrians))

(event EventTick
  (params (DeltaSeconds :type Float%20%28single-precision%29))
  (bind _gametime (CallFunction|GetGameTime))
  (CallFunction|SetGameStage _gametime))

(fn ConstructionScript)

(fn SetReferencesandSpawnLocations
  (Utilities|FlowControl|DoOnce false
    (:Completed
      (bind _outactors (Actor|GetAllActorsOfClass "/Game/VehicleAdvBP/Blueprints/VehicleBlueprint.VehicleBlueprint_C"))
      (Variables|Default|SetPlayer_Ref (Utilities|Array|Get(acopy) _outactors))
      (bind _returnvalue (Actor|GetActorOfClass "/Game/MyContent/Blueprints/Actors/BP_SpawnPoint_A.BP_SpawnPoint_A_C"))
      (bind _output_get (Variables|Default|SetSpawnPoint_A_Ref _returnvalue))
      (Variables|Default|SetSpawnPointLocation_A (Transformation|GetActorLocation _output_get))
      (bind _returnvalue_2 (Actor|GetActorOfClass "/Game/MyContent/Blueprints/Actors/BP_SpawnPoint_B.BP_SpawnPoint_B_C"))
      (bind _output_get_2 (Variables|Default|SetSpawnPoint_B_Ref _returnvalue_2))
      (Variables|Default|SetSpawnPointLocation_B (Transformation|GetActorLocation _output_get_2))
      (bind _returnvalue_3 (Game|GetCurrentLevelName true))
      (Variables|Default|SetCurrentLevelName _returnvalue_3)
      (CallFunction|SetMaxGameStage)
      (return))))

(fn SetMaxGameStage
  (Variables|Default|SetMaxGameStage (Utilities|Array|Length (Variables|Default|GetGameStageLengths)))
  (return))

(fn SetPedestrianSpawnTransform
  (bind _spawnpointlocation_a (Variables|Default|GetSpawnPointLocation_A))
  (bind _spawnpointlocation_a_2 (Variables|Default|GetSpawnPointLocation_A))
  (bind _spawnpointlocation_b (Variables|Default|GetSpawnPointLocation_B))
  (bind _streetwidth (Variables|Default|GetStreetWidth))
  (bind _streetwidth_2 (Variables|Default|GetStreetWidth))
  (bind _spawnpointlocation_b_2 (Variables|Default|GetSpawnPointLocation_B))
  (bind _returnvalue (/ _streetwidth 2.0))
  (bind _returnvalue_2 (/ _streetwidth_2 2.0))
  (if (Math|Random|RandomBool)
    (LocalVariables|SetSpawnRotation_Loc "0, 0, 0")
    (bind _output_get (LocalVariables|SetSpawnTransform_Loc (Math|Transform|MakeTransform (Math|Vector|MakeVector (Math|Random|RandomFloatinRange (- (.x _spawnpointlocation_a) _returnvalue_2) (+ (.x _spawnpointlocation_a) _returnvalue_2)) (.y _spawnpointlocation_a) (Variables|Default|GetPedestrianHalfHeight)) (LocalVariables|GetSpawnRotation_Loc) "1,1,1")))
    (bind _output_get_2 (LocalVariables|SetTargetLocation_Loc (Math|Vector|MakeVector (.x (.location _output_get)) (.y _spawnpointlocation_b_2) (.z _spawnpointlocation_b_2))))
    (return _output_get_2 (LocalVariables|GetSpawnTransform_Loc))
    (else
      (LocalVariables|SetSpawnRotation_Loc "0, 0, 0")
      (bind _output_get_3 (LocalVariables|SetSpawnTransform_Loc (Math|Transform|MakeTransform (Math|Vector|MakeVector (Math|Random|RandomFloatinRange (- (.x _spawnpointlocation_b) _returnvalue) (+ (.x _spawnpointlocation_b) _returnvalue)) (.y _spawnpointlocation_b) (Variables|Default|GetPedestrianHalfHeight)) (LocalVariables|GetSpawnRotation_Loc) "1,1,1")))
      (bind _output_get_4 (LocalVariables|SetTargetLocation_Loc (Math|Vector|MakeVector (.x (.location _output_get_3)) (.y _spawnpointlocation_a_2) (.z _spawnpointlocation_a_2))))
      (return _output_get_4 (LocalVariables|GetSpawnTransform_Loc)))))

(fn SpawnPedestrians
  (bind (_targetlocation _spawntransform) (CallFunction|SetPedestrianSpawnTransform :!label _label))
  (bind _returnvalue (Game|SpawnActorfromClass "/Game/MyContent/Blueprints/Characters/BP_Pedestrian.BP_Pedestrian_C" _spawntransform "AdjustIfPossibleButAlwaysSpawn" 0 false false false false _targetlocation false false 0))
  (Utilities|Array|Add (Variables|/Game/VehicleAdvBP/Blueprints/VehicleBlueprint.VehicleBlueprint_C|GetPedestrian_Refs (Variables|Default|GetPlayer_Ref)) _returnvalue)
  (bind _result (Math|Integer|IncrementInt (Variables|Default|GetPedestrianID))
    (:%20%20
      (bind _output_get (Variables|Default|SetPedestrianID _result))
      (Utilities|Array|Add (Variables|/Script/Engine.Actor|GetTags _returnvalue) (Utilities|String|StringToName (Utilities|String|ToString(Integer) _output_get)))
      (bind _pedestrianstospawn_ (CallFunction|SetPedestrianNumberSpawned))
      (if _pedestrianstospawn_
        (goto _label)
        (else
          (return))))))

(fn SetPedestrianNumberSpawned
  (bind _result (Math|Integer|IncrementInt (Variables|Default|GetPedestrianNumberSpawned))
    (:%20%20
      (bind _output_get (Variables|Default|SetPedestrianNumberSpawned _result))
      (return (< _output_get (Variables|Default|GetPedestrianNumberToSpawn))))))

(fn GetGameTime
  (if (Utilities|Enum|Equal(Enum) (Variables|Default|GetCurrentLevelName) (Variables|Default|GetTargetLevelName))
    (return (Utilities|Time|GetGameTimeinSeconds))
    (else
      (return 0.0))))

(fn SetGameStage
  (params (GameTime :type Float%20%28single-precision%29))
  (if (== (Math|Float|Round GameTime) (Utilities|Array|Get(acopy) (Variables|Default|GetGameStageLengths) (Variables|Default|GetGameStage)))
    (bind _result (Math|Integer|IncrementInt (Variables|Default|GetGameStage))
      (:%20%20
        (if (>= (Variables|Default|GetMaxGameStage) _result)
          (Variables|Default|SetGameStage _result)))))
  (return))
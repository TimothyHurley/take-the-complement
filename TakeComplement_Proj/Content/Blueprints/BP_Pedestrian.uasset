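; BP_Pedestrian is an AI pedestrian that moves toward the player once its PawnSensing component sees a pawn.
; Any sighting calls FollowPlayer, which runs AIMoveTo on player character 0 and prints debug text on success or failure; its IsFollowingPlayer branch is empty.
; SetTargetPosition, uncalled here, sets TargetPosition from the spawn location with Y zeroed, ignoring its index branch.
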(event OnSeePawn(PawnSensing)
  (params (Pawn :type Pawn%20Object%20Reference))
  (CallFunction|FollowPlayer))

(event Custom|FollowPlayer
  (if (Variables|Default|GetIsFollowingPlayer?)
    _
    (else
      _))
  (AI|AIMoveTo self "0, 0, 0" (Game|GetPlayerCharacter 0) 5.0 false
    (:OnSuccess
      (Development|PrintString "Hello"))
    (:OnFail
      (Development|PrintString "Goodbye"))))

(event EventBeginPlay)

(event Collision|EventActorBeginOverlap
  (params (OtherActor :type Actor%20Object%20Reference)))

(event EventTick
  (params (DeltaSeconds :type Float%20%28single-precision%29)))

(fn ConstructionScript)

(fn SetTargetPosition
  (params (OtherTargetPointIndex :type Integer) (SpawnTransform :type Transform))
  (if (== OtherTargetPointIndex 0)
    _
    (else
      _))
  (Variables|Default|SetTargetPosition (Math|Vector|MakeVector (.x (.location SpawnTransform)) 0.0 (.z (.location SpawnTransform))))
  (return))
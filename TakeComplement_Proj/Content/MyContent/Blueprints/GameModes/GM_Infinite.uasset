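; Game mode for an infinite mode that populates a street with pedestrians and tracks timed stages.
; On BeginPlay it caches the player vehicle and two spawn points, then spawns a set number of pedestrians randomly across either end, targeting the opposite end.
; Each pedestrian gets an ID tag and is registered on the vehicle.
; Tick advances and prints the stage when rounded game time equals the current StageLengths entry.
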(event EventBeginPlay
  (bind _outactors (Actor|GetAllActorsOfClass "/Game/VehicleAdvBP/Blueprints/VehicleBlueprint.VehicleBlueprint_C"))
  (Variables|Default|SetPlayer_Ref (Utilities|Array|Get(acopy) _outactors))
  (CallFunction|SetPedestrianSpawnPoints)
  (CallFunction|SpawnPedestrians)
  (Variables|Default|SetMaxStage (Utilities|Array|Length (Variables|Default|GetStageLengths))))

(event EventTick
  (params (DeltaSeconds :type Float%20%28single-precision%29))
  (if (== (Math|Float|Round (Utilities|Time|GetGameTimeinSeconds)) (Utilities|Array|Get(acopy) (Variables|Default|GetStageLengths) (Variables|Default|GetStage)))
    (bind _result (Math|Integer|IncrementInt (Variables|Default|GetStage))
      (:%20%20
        (bind _output_get (Variables|Default|SetStage _result))
        (Development|PrintString (Utilities|String|ToString(Integer) _output_get))))))

(fn ConstructionScript)

(fn SetPedestrianSpawnPoints
  (bind _returnvalue (Actor|GetActorOfClass "/Game/MyContent/Blueprints/Actors/BP_SpawnPoint_A.BP_SpawnPoint_A_C"))
  (bind _output_get (Variables|Default|SetSpawnPoint_A_Ref _returnvalue))
  (Variables|Default|SetSpawnPointLocation_A (Transformation|GetActorLocation _output_get))
  (bind _returnvalue_2 (Actor|GetActorOfClass "/Game/MyContent/Blueprints/Actors/BP_SpawnPoint_B.BP_SpawnPoint_B_C"))
  (bind _output_get_2 (Variables|Default|SetSpawnPoint_B_Ref _returnvalue_2))
  (Variables|Default|SetSpawnPointLocation_B (Transformation|GetActorLocation _output_get_2))
  (return))

(fn SpawnPedestrians
  (CallFunction|SetPedestrianSpawnTransform :!label _label)
  (bind _returnvalue (Game|SpawnActorfromClass "/Game/MyContent/Blueprints/Characters/BP_Pedestrian.BP_Pedestrian_C" (Variables|Default|GetSpawnTransform) "AdjustIfPossibleButAlwaysSpawn" 0 false false false (Variables|Default|GetTargetPointLocation) 0))
  (Utilities|Array|Add (Variables|/Game/VehicleAdvBP/Blueprints/VehicleBlueprint.VehicleBlueprint_C|GetPedestrian_Refs (Variables|Default|GetPlayer_Ref)) _returnvalue)
  (bind _result (Math|Integer|IncrementInt (Variables|Default|GetPedestrianID))
    (:%20%20
      (bind _output_get (Variables|Default|SetPedestrianID _result))
      (Utilities|Array|Add (Variables|/Script/Engine.Actor|GetTags _returnvalue) (Utilities|String|StringToName (Utilities|String|ToString(Integer) _output_get)))
      (bind _pedestrianstospawn_ (CallFunction|UpdatePedestrianNumberSpawned))
      (if _pedestrianstospawn_
        (goto _label)
        (else
          (return))))))

(fn SetPedestrianSpawnTransform
  (bind _spawnpointlocation_a (Variables|Default|GetSpawnPointLocation_A))
  (bind _spawnpointlocation_a_2 (Variables|Default|GetSpawnPointLocation_A))
  (bind _spawnpointlocation_b (Variables|Default|GetSpawnPointLocation_B))
  (bind _streetwidth (Variables|Default|GetStreetWidth))
  (bind _streetwidth_2 (Variables|Default|GetStreetWidth))
  (bind _spawnpointlocation_b_2 (Variables|Default|GetSpawnPointLocation_B))
  (bind _returnvalue (/ _streetwidth 2.0))
  (bind _returnvalue_2 (/ _streetwidth_2 2.0))
  (if (Math|Random|RandomBool)
    (LocalVariables|SetSpawnRotation "0, 0, 0")
    (Variables|Default|SetSpawnTransform (Math|Transform|MakeTransform (Math|Vector|MakeVector (Math|Random|RandomFloatinRange (- (.x _spawnpointlocation_a) _returnvalue_2) (+ (.x _spawnpointlocation_a) _returnvalue_2)) (.y _spawnpointlocation_a) (Variables|Default|GetPedestrianHalfHeight)) (LocalVariables|GetSpawnRotation) "1,1,1"))
    (Variables|Default|SetTargetPointLocation (Math|Vector|MakeVector (.x (.location (Variables|Default|GetSpawnTransform))) (.y _spawnpointlocation_b_2) (.z _spawnpointlocation_b_2)))
    (else
      (LocalVariables|SetSpawnRotation "0, 0, 0")
      (Variables|Default|SetSpawnTransform (Math|Transform|MakeTransform (Math|Vector|MakeVector (Math|Random|RandomFloatinRange (- (.x _spawnpointlocation_b) _returnvalue) (+ (.x _spawnpointlocation_b) _returnvalue)) (.y _spawnpointlocation_b) (Variables|Default|GetPedestrianHalfHeight)) (LocalVariables|GetSpawnRotation) "1,1,1"))
      (Variables|Default|SetTargetPointLocation (Math|Vector|MakeVector (.x (.location (Variables|Default|GetSpawnTransform))) (.y _spawnpointlocation_a_2) (.z _spawnpointlocation_a_2)))))
  (return))

(fn UpdatePedestrianNumberSpawned
  (bind _result (Math|Integer|IncrementInt (Variables|Default|GetPedestrianNumberSpawned))
    (:%20%20
      (bind _output_get (Variables|Default|SetPedestrianNumberSpawned _result))
      (return (< _output_get (Variables|Default|GetPedestrianNumberToSpawn))))))
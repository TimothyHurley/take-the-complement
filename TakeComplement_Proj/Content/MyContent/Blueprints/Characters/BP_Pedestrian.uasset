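; Pedestrian character that walks to a street destination, or follows the player's vehicle once flagged, until beyond ComplementRange.
; Tick reissues AI moves, or halts movement while stunned, setting custom depth stencil values by state.
; Overlap volumes handle stunning, too-close detection, and ending gameplay with a menu when a follower reaches the player.
; Losing range banks the HUD score streak; arriving destroys the pedestrian and requests a respawn from GM_Infinite.
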(event OnComponentBeginOverlap(CollisionSphere_TooClose)
  (params (OverlappedComponent :type Primitive%20Component%20Object%20Reference) (OtherActor :type Actor%20Object%20Reference) (OtherComp :type Primitive%20Component%20Object%20Reference) (OtherBodyIndex :type Integer) (bFromSweep :type Boolean) (SweepResult :type Hit%20Result%20Structure%20%28by%20ref%29))
  (if (== (Variables|Default|GetPlayer_Ref) OtherActor)
    (Variables|Default|SetIsTooClose? true)))

(event OnComponentEndOverlap(CollisionSphere_TooClose)
  (params (OverlappedComponent :type Primitive%20Component%20Object%20Reference) (OtherActor :type Actor%20Object%20Reference) (OtherComp :type Primitive%20Component%20Object%20Reference) (OtherBodyIndex :type Integer))
  (if (== (Variables|Default|GetPlayer_Ref) OtherActor)
    (Variables|Default|SetIsTooClose? false)))

(event OnComponentBeginOverlap(CapsuleComponent)
  (params (OverlappedComponent :type Primitive%20Component%20Object%20Reference) (OtherActor :type Actor%20Object%20Reference) (OtherComp :type Primitive%20Component%20Object%20Reference) (OtherBodyIndex :type Integer) (bFromSweep :type Boolean) (SweepResult :type Hit%20Result%20Structure%20%28by%20ref%29))
  (if (== (Variables|Default|GetPlayer_Ref) OtherActor)
    (Variables|/Game/VehicleAdvBP/Blueprints/VehicleBlueprint.VehicleBlueprint_C|SetIsPedestrianStunned? (Variables|Default|GetPlayer_Ref) true)
    (Variables|Default|SetIsStunned? true)
    (Variables|Default|SetIsTooClose? false)))

(event OnComponentBeginOverlap(CollisionSphere_Thank)
  (params (OverlappedComponent :type Primitive%20Component%20Object%20Reference) (OtherActor :type Actor%20Object%20Reference) (OtherComp :type Primitive%20Component%20Object%20Reference) (OtherBodyIndex :type Integer) (bFromSweep :type Boolean) (SweepResult :type Hit%20Result%20Structure%20%28by%20ref%29))
  (if (and (== (Variables|Default|GetPlayer_Ref) OtherActor) (Variables|Default|GetIsFollowingPlayer?))
    (Default|StopGameplayandCreateMenu (Variables|Default|GetPlayer_Ref))))

(event Custom|FollowPlayer
  (bind _player_ref (Variables|Default|GetPlayer_Ref))
  (AI|AIMoveTo self "0, 0, 0" (Variables|Default|GetPlayer_Ref) 5.0 false
    (:then
      (if (> (Math|Vector|Distance(Vector) (Transformation|GetActorLocation self) (Transformation|GetActorLocation _player_ref)) (* (Variables|/Game/VehicleAdvBP/Blueprints/VehicleBlueprint.VehicleBlueprint_C|GetComplementRange _player_ref) 1.0))
        (CallFunction|ResettoFollowStreet)))))

(event Custom|FollowStreet
  (AI|AIMoveTo self (Variables|Default|GetTargetLocation) 0 5.0 false
    (:OnSuccess
      (Utilities|FlowControl|DoOnce false
        (:Completed
          (CallFunction|DestroySelf)
          (Default|SpawnPedestrians (Variables|Default|GetGameMode_Ref)))))))

(event EventBeginPlay
  (Utilities|FlowControl|Delay 0.05)
  (CallFunction|SetReferences))

(event EventTick
  (params (DeltaSeconds :type Float%20%28single-precision%29))
  (if (Variables|Default|GetIsStunned?)
    (Components|Movement|StopMovementImmediately (Variables|Character|GetCharacterMovement))
    (Rendering|SetCustomDepthStencilValue (Variables|Character|GetMesh) 4)
    (elif (Variables|Default|GetIsFollowingPlayer?)
      (CallFunction|FollowPlayer)
      (else
        (CallFunction|FollowStreet)
        (if (not (Variables|Default|GetIsTargetReference?))
          (Rendering|SetCustomDepthStencilValue (Variables|Character|GetMesh) 0))))))

(fn ConstructionScript)

(fn SetReferences
  (bind _returnvalue (Actor|GetActorOfClass "/Game/MyContent/Blueprints/GameModes/GM_Infinite.GM_Infinite_C"))
  (Variables|Default|SetGameMode_Ref _returnvalue)
  (bind _foundwidgets (Widget|GetAllWidgetsOfClass "/Game/MyContent/Blueprints/Widgets/Game/W_HUD.W_HUD_C" true))
  (Variables|Default|SetHUD_Ref (Utilities|Array|Get(acopy) _foundwidgets))
  (bind _returnvalue_2 (Actor|GetActorOfClass "/Game/VehicleAdvBP/Blueprints/VehicleBlueprint.VehicleBlueprint_C"))
  (Variables|Default|SetPlayer_Ref _returnvalue_2)
  (return))

(fn ResettoFollowStreet
  (bind _hud_ref (Variables|Default|GetHUD_Ref))
  (bind _hud_ref_2 (Variables|Default|GetHUD_Ref))
  (bind _w_score (Variables|/Game/MyContent/Blueprints/Widgets/Game/W_HUD.W_HUD_C|GetW_Score _hud_ref))
  (bind _w_scorestreak (Variables|/Game/MyContent/Blueprints/Widgets/Game/W_HUD.W_HUD_C|GetW_ScoreStreak _hud_ref))
  (bind _w_scorecombo (Variables|/Game/MyContent/Blueprints/Widgets/Game/W_HUD.W_HUD_C|GetW_ScoreCombo _hud_ref_2))
  (Variables|Default|SetIsComplemented? false)
  (Variables|Default|SetIsFollowingPlayer? false)
  (Variables|Default|SetIsAddedToScoreCombo? false)
  (Variables|Default|SetIsStunned? false)
  (bind _result (Math|Integer|DecrementInt (Variables|/Game/MyContent/Blueprints/Widgets/Game/W_ScoreCombo.W_ScoreCombo_C|GetScoreCombo _w_scorecombo))
    (:%20%20
      (Variables|/Game/MyContent/Blueprints/Widgets/Game/W_ScoreCombo.W_ScoreCombo_C|SetScoreCombo _w_scorecombo _result)
      (Variables|/Game/MyContent/Blueprints/Widgets/Game/W_ScoreStreak.W_ScoreStreak_C|SetIsIncreasing? _w_scorestreak false)
      (bind _increasedscore (Default|AddScoreStreaktoScore _w_scorestreak (Variables|/Game/MyContent/Blueprints/Widgets/Game/W_Score.W_Score_C|GetScore _w_score)))
      (Variables|/Game/MyContent/Blueprints/Widgets/Game/W_Score.W_Score_C|SetScore _w_score _increasedscore)
      (Variables|/Game/MyContent/Blueprints/Widgets/Game/W_ScoreStreak.W_ScoreStreak_C|SetStreak (Variables|/Game/MyContent/Blueprints/Widgets/Game/W_HUD.W_HUD_C|GetW_ScoreStreak (Variables|Default|GetHUD_Ref)) 0)
      (return))))

(fn DestroySelf
  (bind _gamemode_ref (Variables|Default|GetGameMode_Ref))
  (Actor|DestroyActor)
  (bind _result (Math|Integer|DecrementInt (Variables|/Game/MyContent/Blueprints/GameModes/GM_Infinite.GM_Infinite_C|GetPedestrianNumberSpawned _gamemode_ref))
    (:%20%20
      (Variables|/Game/MyContent/Blueprints/GameModes/GM_Infinite.GM_Infinite_C|SetPedestrianNumberSpawned _gamemode_ref _result)
      (Utilities|Array|RemoveItem (Variables|/Game/VehicleAdvBP/Blueprints/VehicleBlueprint.VehicleBlueprint_C|GetPedestrian_Refs (Variables|Default|GetPlayer_Ref)) self)
      (if (Utilities|Enum|Equal(Enum) (Utilities|GetDisplayName self) (Utilities|GetDisplayName (Variables|/Game/VehicleAdvBP/Blueprints/VehicleBlueprint.VehicleBlueprint_C|GetTargetPedestrian_Ref (Variables|Default|GetPlayer_Ref))))
        (Variables|/Game/VehicleAdvBP/Blueprints/VehicleBlueprint.VehicleBlueprint_C|SetTargetPedestrian_Ref (Variables|Default|GetPlayer_Ref) 0))
      (return))))
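; Player vehicle pawn where the player aims at pedestrians to "complement" them, recharging a battery and building score combo and streak until the battery runs out.
; Tick rotates the camera and line-traces from it, matching interface-implementing hits to pedestrians by tag.
; Target state drives crosshair, HUD prompt and custom-depth stencil outline.
; Clicking makes valid targets follow, or apologises to stunned ones, clearing the stun flag that divides throttle.
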(event EventBeginPlay
  (CallFunction|CreateHUD)
  (Variables|Default|SetIsPlaying? true)
  (Variables|/Script/Engine.PlayerController|SetbShowMouseCursor (Game|GetPlayerController 0) false))

(event EventTick
  (params (DeltaSeconds :type Float%20%28single-precision%29))
  (if (Variables|Default|GetIsPlaying?)
    (CallFunction|SetPlayerPositionandRotation)
    (if (Variables|/Game/MyContent/Blueprints/Widgets/Game/W_Battery.W_Battery_C|GetIsBatteryEmpty? (Variables|/Game/MyContent/Blueprints/Widgets/Game/W_HUD.W_HUD_C|GetW_Battery (Variables|Default|GetHUD_Ref)))
      (CallFunction|StopGameplayandCreateMenu)
      (else
        (bind (_returnvalue _hitactor) (CallFunction|GetTargetActor (Variables|Default|GetHUD_Ref)))
        (if (Variables|Default|GetIsCrosshairValid?)
          (CallFunction|IdentifyTargetActor _returnvalue _hitactor)
          (CallFunction|SetTargetPedestrian)
          (CallFunction|SetTargetPedestrianState)
          (CallFunction|SetCrosshairState (CallFunction|GetTargetPedestrianValidity))
          (CallFunction|SetTargetPedestrianOutline))))))

(event Input|AxisEvents|InputAxisMoveForward
  (params (AxisValue :type Float%20%28single-precision%29))
  (if (Variables|Default|GetIsPedestrianStunned?)
    (Class|WheeledVehicleMovementComponent|SetThrottleInput (Variables|Default|GetVehicleMovement) (/ AxisValue (Variables|Default|GetMovementSpeedDivisor)))
    (else
      (Class|WheeledVehicleMovementComponent|SetThrottleInput (Variables|Default|GetVehicleMovement) AxisValue))))

(event Input|AxisEvents|InputAxisMoveRight
  (params (AxisValue :type Float%20%28single-precision%29))
  (Class|WheeledVehicleMovementComponent|SetSteeringInput (Variables|Default|GetVehicleMovement) AxisValue))

(event Input|MouseEvents|LeftMouseButton
  (params (Key :type Key%20Structure :default "None"))
  (:Pressed
    (if (CallFunction|GetTargetPedestrianValidity)
      (if (CallFunction|GetCrosshairValidity)
        (if (Variables|/Game/MyContent/Blueprints/Characters/BP_Pedestrian.BP_Pedestrian_C|GetIsStunned? (Variables|Default|GetTargetPedestrian_Ref))
          (CallFunction|ApologisetoPedestrian)
          (elif (not (Variables|/Game/MyContent/Blueprints/Characters/BP_Pedestrian.BP_Pedestrian_C|GetIsTooClose? (Variables|Default|GetTargetPedestrian_Ref)))
            (Variables|Default|SetIsPedestrianHighlighted? true)
            (Variables|/Game/MyContent/Blueprints/Characters/BP_Pedestrian.BP_Pedestrian_C|SetIsFollowingPlayer? (Variables|Default|GetTargetPedestrian_Ref) true)
            (CallFunction|SetPlayerBattery)
            (CallFunction|SetPlayerScoreCombo)
            (CallFunction|SetPlayerScoreStreak)
            (else
              (Variables|Default|SetIsPedestrianHighlighted? false :!label _label)))))
      (else
        (goto _label)))))

(fn ConstructionScript)

(fn CreateHUD
  (bind _returnvalue (UserInterface|CreateWidget "/Game/MyContent/Blueprints/Widgets/Game/W_HUD.W_HUD_C"))
  (bind _output_get (Variables|Default|SetHUD_Ref _returnvalue))
  (UserInterface|Viewport|AddtoViewport _output_get 0)
  (return))

(fn StopGameplayandCreateMenu
  (Utilities|FlowControl|DoOnce false
    (:Completed
      (Variables|Default|SetIsPlaying? false)
      (bind _returnvalue (UserInterface|CreateWidget "/Game/MyContent/Blueprints/Widgets/Menu/W_Menu_Thanks.W_Menu_Thanks_C"))
      (UserInterface|Viewport|AddtoViewport _returnvalue 1)
      (return))))

(fn SetAudioInput
  (Audio|Parameter|SetFloatParameter (Variables|Default|GetEngineSound) "RPM" (Math|Float|Absolute(Float) (Class|WheeledVehicleMovementComponent|GetForwardSpeed (Variables|Default|GetVehicleMovement))) :!class /Script/Engine.AudioComponent))

(fn SetPlayerPositionandRotation
  (bind _camera (Variables|Components|GetCamera))
  (bind _relativerotation (Variables|/Script/Engine.SceneComponent|GetRelativeRotation _camera))
  (bind (_roll _pitch _yaw) (Math|Rotator|BreakRotator _relativerotation))
  (Variables|Default|SetIsReversing? (< (Class|WheeledVehicleMovementComponent|GetCurrentGear (Variables|Default|GetVehicleMovement)) 0))
  (Transformation|SetRelativeRotation (Variables|Components|GetCamera) (Math|Rotator|MakeRotator 0.0 (Math|Float|ClampAngle (+ (Input|AxisValues|GetLookUp) _pitch) -9e+01 9e+01) (+ (Input|AxisValues|GetLookRight) _yaw)) false false)
  (return))

(fn ApologisetoPedestrian
  (Variables|/Game/MyContent/Blueprints/Characters/BP_Pedestrian.BP_Pedestrian_C|SetIsStunned? (Variables|Default|GetTargetPedestrian_Ref) false)
  (Variables|Default|SetIsPedestrianStunned? false)
  (if (Collision|IsOverlappingActor (Variables|Character|GetMesh) (Variables|Default|GetTargetPedestrian_Ref) :!class /Script/Engine.PrimitiveComponent)
    (Variables|/Game/MyContent/Blueprints/Characters/BP_Pedestrian.BP_Pedestrian_C|SetIsTooClose? (Variables|Default|GetTargetPedestrian_Ref) true))
  (return))

(fn SetPlayerBattery
  (bind _targetpedestrian_ref (Variables|Default|GetTargetPedestrian_Ref))
  (if (and (Variables|/Game/MyContent/Blueprints/Characters/BP_Pedestrian.BP_Pedestrian_C|GetIsFollowingPlayer? _targetpedestrian_ref) (not (Variables|/Game/MyContent/Blueprints/Characters/BP_Pedestrian.BP_Pedestrian_C|GetIsComplemented? _targetpedestrian_ref)))
    (Default|IncreaseBatteryPercentage (Variables|/Game/MyContent/Blueprints/Widgets/Game/W_HUD.W_HUD_C|GetW_Battery (Variables|Default|GetHUD_Ref)))
    (Variables|/Game/MyContent/Blueprints/Characters/BP_Pedestrian.BP_Pedestrian_C|SetIsComplemented? (Variables|Default|GetTargetPedestrian_Ref) true))
  (return))

(fn SetPlayerScore)

(fn SetPlayerScoreCombo
  (if (not (Variables|/Game/MyContent/Blueprints/Characters/BP_Pedestrian.BP_Pedestrian_C|GetIsAddedToScoreCombo? (Variables|Default|GetTargetPedestrian_Ref)))
    (Math|Integer|IncrementInt (Variables|/Game/MyContent/Blueprints/Widgets/Game/W_ScoreCombo.W_ScoreCombo_C|GetScoreCombo (Variables|/Game/MyContent/Blueprints/Widgets/Game/W_HUD.W_HUD_C|GetW_ScoreCombo (Variables|Default|GetHUD_Ref)))
      (:%20%20
        (Variables|/Game/MyContent/Blueprints/Characters/BP_Pedestrian.BP_Pedestrian_C|SetIsAddedToScoreCombo? (Variables|Default|GetTargetPedestrian_Ref) true))))
  (return))

(fn SetPlayerScoreStreak
  (if (not (Variables|/Game/MyContent/Blueprints/Widgets/Game/W_ScoreStreak.W_ScoreStreak_C|GetIsIncreasing? (Variables|/Game/MyContent/Blueprints/Widgets/Game/W_HUD.W_HUD_C|GetW_ScoreStreak (Variables|Default|GetHUD_Ref))))
    (Variables|/Game/MyContent/Blueprints/Widgets/Game/W_ScoreStreak.W_ScoreStreak_C|SetIsIncreasing? (Variables|/Game/MyContent/Blueprints/Widgets/Game/W_HUD.W_HUD_C|GetW_ScoreStreak (Variables|Default|GetHUD_Ref)) true))
  (return))

(fn GetTargetActor
  (params (HUD_Ref :type W%20HUD%20Object%20Reference))
  (bind _camera (Variables|Components|GetCamera))
  (bind _returnvalue (Transformation|GetWorldLocation _camera))
  (Variables|/Game/MyContent/Blueprints/Widgets/Game/W_HUD.W_HUD_C|GetW_Crosshair HUD_Ref
    (:then
      (Variables|Default|SetIsCrosshairValid? true)
      (bind (_outhit _returnvalue_2) (Collision|LineTraceByChannel _returnvalue (+ _returnvalue (* (Math|Vector|GetForwardVector _camera) (Variables|Default|GetComplementRange))) "TraceTypeQuery2" false 0 "None")))
    (:else
      (Variables|Default|SetIsCrosshairValid? false)))
  (return _returnvalue_2 (.HitActor (Collision|BreakHitResult _outhit))))

(fn IdentifyTargetActor
  (params (ReturnValue :type Boolean) (HitActor :type Actor%20Object%20Reference))
  (if ReturnValue
    (if (Utilities|DoesObjectImplementInterface HitActor "/Game/MyContent/Blueprints/Interfaces/BP_ComplementInterface.BP_ComplementInterface_C")
      (Variables|Default|SetPedestrianID_Ref (Utilities|Array|Get(acopy) (Variables|/Script/Engine.Actor|GetTags HitActor)))
      (Variables|Default|SetIsInComplementRange? true)
      (else
        (Variables|Default|SetPedestrianID_Ref "None" :!label _label)
        (Variables|Default|SetIsInComplementRange? false)))
    (else
      (goto _label)))
  (return))

(fn SetTargetPedestrian
  (for _array_element (Variables|Default|GetPedestrian_Refs)
    (Variables|/Game/MyContent/Blueprints/Characters/BP_Pedestrian.BP_Pedestrian_C|SetIsTargetReference? _array_element false))
  (if (Variables|Default|GetIsInComplementRange?)
    (bind _array_element_2 (Utilities|Array|ForEachLoopwithBreak (Variables|Default|GetPedestrian_Refs) :!label _label)
      (:LoopBody
        (if (Utilities|Name|Equal(Name) (Utilities|Array|Get(acopy) (Variables|/Script/Engine.Actor|GetTags _array_element_2)) (Variables|Default|GetPedestrianID_Ref))
          (bind _output_get (Variables|Default|SetTargetPedestrian_Ref _array_element_2))
          (Variables|/Game/MyContent/Blueprints/Characters/BP_Pedestrian.BP_Pedestrian_C|SetIsTargetReference? _output_get true)
          (goto _label Break)
          (else
            (Variables|Default|SetTargetPedestrian_Ref 0)
            (Variables|/Game/MyContent/Blueprints/Characters/BP_Pedestrian.BP_Pedestrian_C|SetIsTargetReference? _array_element_2 false))))
      (:Completed
        (return)))
    (else
      (return))))

(fn SetCrosshairState
  (params (IsValid? :type Boolean))
  (if IsValid?
    (if (not (Utilities|Name|Equal(Name) (Variables|Default|GetPedestrianID_Ref) "None"))
      (if (Variables|/Game/MyContent/Blueprints/Characters/BP_Pedestrian.BP_Pedestrian_C|GetIsTooClose? (Variables|Default|GetTargetPedestrian_Ref))
        (if (CallFunction|GetCrosshairValidity)
          _
          (else
            (UserInterface|Viewport|AddtoViewport (Variables|/Game/MyContent/Blueprints/Widgets/Game/W_HUD.W_HUD_C|GetW_Crosshair (Variables|Default|GetHUD_Ref)) 0)))
        (elif (CallFunction|GetCrosshairValidity)
          _
          (else
            (UserInterface|Viewport|AddtoViewport (Variables|/Game/MyContent/Blueprints/Widgets/Game/W_HUD.W_HUD_C|GetW_Crosshair (Variables|Default|GetHUD_Ref)) 0))))
      (else
        (if (CallFunction|GetCrosshairValidity) :!label _label
          (Widget|RemovefromParent (Variables|/Game/MyContent/Blueprints/Widgets/Game/W_HUD.W_HUD_C|GetW_Crosshair (Variables|Default|GetHUD_Ref))))))
    (else
      (goto _label)))
  (return))

(fn SetTargetPedestrianState
  (bind _targetpedestrian_ref (Variables|Default|GetTargetPedestrian_Ref))
  (if (CallFunction|GetTargetPedestrianValidity)
    (if (Variables|/Game/MyContent/Blueprints/Characters/BP_Pedestrian.BP_Pedestrian_C|GetIsStunned? (Variables|Default|GetTargetPedestrian_Ref))
      (Variables|Default|SetOutlineStencilValue 4)
      (Default|SetStunned (Variables|/Game/MyContent/Blueprints/Widgets/Game/W_HUD.W_HUD_C|GetW_ComplementPrompt (Variables|Default|GetHUD_Ref)))
      (if (CallFunction|GetCrosshairValidity)
        _
        (else
          (Default|SetOutOfRange (Variables|/Game/MyContent/Blueprints/Widgets/Game/W_HUD.W_HUD_C|GetW_ComplementPrompt (Variables|Default|GetHUD_Ref)))))
      (elif (Variables|/Game/MyContent/Blueprints/Characters/BP_Pedestrian.BP_Pedestrian_C|GetIsFollowingPlayer? (Variables|Default|GetTargetPedestrian_Ref))
        (Variables|Default|SetOutlineStencilValue 3)
        (Default|SetFollowing (Variables|/Game/MyContent/Blueprints/Widgets/Game/W_HUD.W_HUD_C|GetW_ComplementPrompt (Variables|Default|GetHUD_Ref)))
        (elif (CallFunction|GetCrosshairValidity)
          (if (Variables|/Game/MyContent/Blueprints/Characters/BP_Pedestrian.BP_Pedestrian_C|GetIsTooClose? (Variables|Default|GetTargetPedestrian_Ref))
            (Variables|Default|SetOutlineStencilValue 2)
            (Default|SetTooClose (Variables|/Game/MyContent/Blueprints/Widgets/Game/W_HUD.W_HUD_C|GetW_ComplementPrompt (Variables|Default|GetHUD_Ref)))
            (else
              (Variables|Default|SetOutlineStencilValue 1)
              (Default|SetinRange (Variables|/Game/MyContent/Blueprints/Widgets/Game/W_HUD.W_HUD_C|GetW_ComplementPrompt (Variables|Default|GetHUD_Ref)))))
          (elif (not (and (Variables|/Game/MyContent/Blueprints/Characters/BP_Pedestrian.BP_Pedestrian_C|GetIsStunned? _targetpedestrian_ref) (Variables|/Game/MyContent/Blueprints/Characters/BP_Pedestrian.BP_Pedestrian_C|GetIsFollowingPlayer? _targetpedestrian_ref)))
            (Variables|Default|SetOutlineStencilValue 0)
            (Default|SetOutOfRange (Variables|/Game/MyContent/Blueprints/Widgets/Game/W_HUD.W_HUD_C|GetW_ComplementPrompt (Variables|Default|GetHUD_Ref))))))))
  (return))

(fn SetTargetPedestrianOutline
  (bind _targetpedestrian_ref (Variables|Default|GetTargetPedestrian_Ref))
  (bind _targetpedestrian_ref_2 (Variables|Default|GetTargetPedestrian_Ref))
  (if (CallFunction|GetCrosshairValidity)
    (Rendering|SetCustomDepthStencilValue (Variables|/Script/Engine.Character|GetMesh _targetpedestrian_ref_2) (Variables|Default|GetOutlineStencilValue) :!label _label)
    (if (Variables|/Game/MyContent/Blueprints/Characters/BP_Pedestrian.BP_Pedestrian_C|GetIsStunned? _targetpedestrian_ref_2)
      (bind _output_get (Variables|Default|SetOutlineStencilValue 4))
      (Rendering|SetCustomDepthStencilValue (Variables|/Script/Engine.Character|GetMesh _targetpedestrian_ref) _output_get)
      (Components|Movement|StopMovementImmediately (Variables|/Script/Engine.Character|GetCharacterMovement _targetpedestrian_ref)))
    (elif (not (Utilities|Enum|Equal(Enum) (Utilities|GetDisplayName (Variables|Default|GetTargetPedestrian_Ref)) ""))
      (if (< (Variables|Default|GetOutlineStencilValue) 2)
        (goto _label)
        (else
          _))))
  (return))

(fn GetCrosshairValidity
  (if (UserInterface|Viewport|IsinViewport (Variables|/Game/MyContent/Blueprints/Widgets/Game/W_HUD.W_HUD_C|GetW_Crosshair (Variables|Default|GetHUD_Ref)))
    (return true)
    (else
      (return false))))

(fn GetTargetPedestrianValidity
  (if (Utilities|Enum|Equal(Enum) (Utilities|GetDisplayName (Variables|Default|GetTargetPedestrian_Ref)) "")
    (Variables|Default|SetTargetPedestrian_Ref 0)
    (return false)
    (else
      (return true))))
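; Game mode for infinite play that keeps spawning pedestrians, each given a random name and registered with the player.
; On the target level, BeginPlay caches references and spawn points, spawns an initial batch and pauses for a tutorial on first start.
; Each pedestrian starts randomly across one of four streets' widths, targeting the opposite end.
; A Delay on Tick paces ongoing spawns, while a looping timer rescales the maximum delay by a divisor.
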(event Custom|DecreaseSpawnDelay
  (Variables|Default|SetSpawnDelay (Math|Float|Clamp(Float) (/ (Variables|Default|GetSpawnDelay) (Variables|Default|GetSpawnDelayDivisor)) 1.0 (Variables|Default|GetMaxSpawnDelay))))

(event EventBeginPlay
  (if (CallFunction|GetCurrentLevelName)
    (CallFunction|SetReferences)
    (CallFunction|SetPedestrianSpawnLocations)
    (CallFunction|SpawnInitialPedestrians)
    (if (Variables|Default|GetIsFirstStart?)
      (Utilities|FlowControl|Delay 0.15)
      (Variables|Default|SetIsFirstStart? false)
      (Default|PauseGameplay (Variables|References|GetPlayer_Ref) true false false false false))
    (Utilities|Time|SetTimerbyEvent (delegate Custom|DecreaseSpawnDelay) 15.0 true)))

(event EventTick
  (params (DeltaSeconds :type Float%20%28single-precision%29))
  (Utilities|FlowControl|Delay (Math|Random|RandomFloatinRange 1.0 (Variables|Default|GetSpawnDelay)))
  (CallFunction|SpawnPedestrian)
  (CallFunction|IncreasePedestrianNumberSpawned))

(fn ConstructionScript)

(fn SetReferences
  (bind _outactors (Actor|GetAllActorsOfClass "/Game/MyContent/Blueprints/Players/BP_Player.BP_Player_C"))
  (Variables|References|SetPlayer_Ref (Utilities|Array|Get(acopy) _outactors))
  (bind _foundwidgets (Widget|GetAllWidgetsOfClass "/Game/MyContent/Blueprints/Widgets/HUD/W_HUD.W_HUD_C" true))
  (Variables|References|SetHUD_Ref (Utilities|Array|Get(acopy) _foundwidgets))
  (Variables|Default|SetSpawnDelay (Variables|Default|GetMaxSpawnDelay))
  (return))

(fn SetPedestrianSpawnLocations
  (bind _returnvalue (Actor|GetActorOfClass "/Game/MyContent/Blueprints/Actors/SpawnPoints/BP_SpawnPoint_A.BP_SpawnPoint_A_C"))
  (bind _output_get (Variables|SpawnPoints|SetSpawnPoint_A_Ref _returnvalue))
  (Variables|SpawnPointLocations|SetSpawnPointLocation_A (Transformation|GetActorLocation _output_get))
  (bind _returnvalue_2 (Actor|GetActorOfClass "/Game/MyContent/Blueprints/Actors/SpawnPoints/BP_SpawnPoint_B.BP_SpawnPoint_B_C"))
  (bind _output_get_2 (Variables|SpawnPoints|SetSpawnPoint_B_Ref _returnvalue_2))
  (Variables|SpawnPointLocations|SetSpawnPointLocation_B (Transformation|GetActorLocation _output_get_2))
  (bind _returnvalue_3 (Actor|GetActorOfClass "/Game/MyContent/Blueprints/Actors/SpawnPoints/BP_SpawnPoint_C.BP_SpawnPoint_C_C"))
  (bind _output_get_3 (Variables|SpawnPoints|SetSpawnPoint_C_Ref _returnvalue_3))
  (Variables|SpawnPointLocations|SetSpawnPointLocation_C (Transformation|GetActorLocation _output_get_3))
  (bind _returnvalue_4 (Actor|GetActorOfClass "/Game/MyContent/Blueprints/Actors/SpawnPoints/BP_SpawnPoint_D.BP_SpawnPoint_D_C"))
  (bind _output_get_4 (Variables|SpawnPoints|SetSpawnPoint_D_Ref _returnvalue_4))
  (Variables|SpawnPointLocations|SetSpawnPointLocation_D (Transformation|GetActorLocation _output_get_4))
  (bind _returnvalue_5 (Actor|GetActorOfClass "/Game/MyContent/Blueprints/Actors/SpawnPoints/BP_SpawnPoint_E.BP_SpawnPoint_E_C"))
  (bind _output_get_5 (Variables|SpawnPoints|SetSpawnPoint_E_Ref _returnvalue_5))
  (Variables|SpawnPointLocations|SetSpawnPointLocation_E (Transformation|GetActorLocation _output_get_5))
  (bind _returnvalue_6 (Actor|GetActorOfClass "/Game/MyContent/Blueprints/Actors/SpawnPoints/BP_SpawnPoint_F.BP_SpawnPoint_F_C"))
  (bind _output_get_6 (Variables|SpawnPoints|SetSpawnPoint_F_Ref _returnvalue_6))
  (Variables|SpawnPointLocations|SetSpawnPointLocation_F (Transformation|GetActorLocation _output_get_6))
  (bind _returnvalue_7 (Actor|GetActorOfClass "/Game/MyContent/Blueprints/Actors/SpawnPoints/BP_SpawnPoint_G.BP_SpawnPoint_G_C"))
  (bind _output_get_7 (Variables|SpawnPoints|SetSpawnPoint_G_Ref _returnvalue_7))
  (Variables|SpawnPointLocations|SetSpawnPointLocation_G (Transformation|GetActorLocation _output_get_7))
  (bind _returnvalue_8 (Actor|GetActorOfClass "/Game/MyContent/Blueprints/Actors/SpawnPoints/BP_SpawnPoint_H.BP_SpawnPoint_H_C"))
  (bind _output_get_8 (Variables|SpawnPoints|SetSpawnPoint_H_Ref _returnvalue_8))
  (Variables|SpawnPointLocations|SetSpawnPointLocation_H (Transformation|GetActorLocation _output_get_8))
  (return))

(fn SetPedestrianSpawnTransform
  (bind _streetwidth (Variables|Default|GetStreetWidth))
  (bind _streetwidth_2 (Variables|Default|GetStreetWidth))
  (bind _spawnpointlocation_c (Variables|SpawnPointLocations|GetSpawnPointLocation_C))
  (bind _spawnpointlocation_d (Variables|SpawnPointLocations|GetSpawnPointLocation_D))
  (bind _spawnpointlocation_c_2 (Variables|SpawnPointLocations|GetSpawnPointLocation_C))
  (bind _spawnpointlocation_d_2 (Variables|SpawnPointLocations|GetSpawnPointLocation_D))
  (bind _streetwidth_3 (Variables|Default|GetStreetWidth))
  (bind _streetwidth_4 (Variables|Default|GetStreetWidth))
  (bind _streetwidth_5 (Variables|Default|GetStreetWidth))
  (bind _spawnpointlocation_a (Variables|SpawnPointLocations|GetSpawnPointLocation_A))
  (bind _spawnpointlocation_a_2 (Variables|SpawnPointLocations|GetSpawnPointLocation_A))
  (bind _spawnpointlocation_b (Variables|SpawnPointLocations|GetSpawnPointLocation_B))
  (bind _spawnpointlocation_b_2 (Variables|SpawnPointLocations|GetSpawnPointLocation_B))
  (bind _streetwidth_6 (Variables|Default|GetStreetWidth))
  (bind _streetwidth_7 (Variables|Default|GetStreetWidth))
  (bind _spawnpointlocation_e (Variables|SpawnPointLocations|GetSpawnPointLocation_E))
  (bind _spawnpointlocation_f (Variables|SpawnPointLocations|GetSpawnPointLocation_F))
  (bind _spawnpointlocation_e_2 (Variables|SpawnPointLocations|GetSpawnPointLocation_E))
  (bind _spawnpointlocation_f_2 (Variables|SpawnPointLocations|GetSpawnPointLocation_F))
  (bind _streetwidth_8 (Variables|Default|GetStreetWidth))
  (bind _spawnpointlocation_g (Variables|SpawnPointLocations|GetSpawnPointLocation_G))
  (bind _spawnpointlocation_h (Variables|SpawnPointLocations|GetSpawnPointLocation_H))
  (bind _spawnpointlocation_g_2 (Variables|SpawnPointLocations|GetSpawnPointLocation_G))
  (bind _spawnpointlocation_h_2 (Variables|SpawnPointLocations|GetSpawnPointLocation_H))
  (bind _returnvalue (/ _streetwidth_3 2.0))
  (bind _returnvalue_2 (/ _streetwidth 2.0))
  (bind _returnvalue_3 (/ _streetwidth_2 2.0))
  (bind _returnvalue_4 (/ _streetwidth_8 2.0))
  (bind _returnvalue_5 (/ _streetwidth_4 2.0))
  (bind _returnvalue_6 (/ _streetwidth_5 2.0))
  (bind _returnvalue_7 (/ _streetwidth_6 2.0))
  (bind _returnvalue_8 (/ _streetwidth_7 2.0))
  (LocalVariables|SetRandomInteger_Loc (Math|Random|RandomInteger 4))
  (if (== (LocalVariables|GetRandomInteger_Loc) 0)
    (if (Math|Random|RandomBool)
      (LocalVariables|SetSpawnRotation_Loc "0, 0, 0")
      (bind _output_get (LocalVariables|SetSpawnTransform_Loc (Math|Transform|MakeTransform (Math|Vector|MakeVector (Math|Random|RandomFloatinRange (- (.x _spawnpointlocation_a_2) _returnvalue_5) (+ (.x _spawnpointlocation_a_2) _returnvalue_5)) (.y _spawnpointlocation_a_2) (Variables|Default|GetPedestrianHalfHeight)) (LocalVariables|GetSpawnRotation_Loc) "1,1,1")))
      (bind _output_get_2 (LocalVariables|SetTargetLocation_Loc (Math|Vector|MakeVector (.x (.location _output_get)) (.y _spawnpointlocation_b_2) (.z _spawnpointlocation_b_2))))
      (return _output_get_2 (LocalVariables|GetSpawnTransform_Loc))
      (else
        (LocalVariables|SetSpawnRotation_Loc "0, 0, 0")
        (bind _output_get_3 (LocalVariables|SetSpawnTransform_Loc (Math|Transform|MakeTransform (Math|Vector|MakeVector (Math|Random|RandomFloatinRange (- (.x _spawnpointlocation_b) _returnvalue_6) (+ (.x _spawnpointlocation_b) _returnvalue_6)) (.y _spawnpointlocation_b) (Variables|Default|GetPedestrianHalfHeight)) (LocalVariables|GetSpawnRotation_Loc) "1,1,1")))
        (bind _output_get_4 (LocalVariables|SetTargetLocation_Loc (Math|Vector|MakeVector (.x (.location _output_get_3)) (.y _spawnpointlocation_a) (.z _spawnpointlocation_a))))
        (return _output_get_4 (LocalVariables|GetSpawnTransform_Loc))))
    (elif (== (LocalVariables|GetRandomInteger_Loc) 1)
      (if (Math|Random|RandomBool)
        (LocalVariables|SetSpawnRotation_Loc "0, 0, 0")
        (bind _output_get_5 (LocalVariables|SetSpawnTransform_Loc (Math|Transform|MakeTransform (Math|Vector|MakeVector (Math|Random|RandomFloatinRange (- (.x _spawnpointlocation_c_2) _returnvalue_4) (+ (.x _spawnpointlocation_c_2) _returnvalue_4)) (.y _spawnpointlocation_c_2) (Variables|Default|GetPedestrianHalfHeight)) (LocalVariables|GetSpawnRotation_Loc) "1,1,1")))
        (bind _output_get_6 (LocalVariables|SetTargetLocation_Loc (Math|Vector|MakeVector (.x (.location _output_get_5)) (.y _spawnpointlocation_d) (.z _spawnpointlocation_d))))
        (return _output_get_6 (LocalVariables|GetSpawnTransform_Loc))
        (else
          (LocalVariables|SetSpawnRotation_Loc "0, 0, 0")
          (bind _output_get_7 (LocalVariables|SetSpawnTransform_Loc (Math|Transform|MakeTransform (Math|Vector|MakeVector (Math|Random|RandomFloatinRange (- (.x _spawnpointlocation_d_2) _returnvalue) (+ (.x _spawnpointlocation_d_2) _returnvalue)) (.y _spawnpointlocation_d_2) (Variables|Default|GetPedestrianHalfHeight)) (LocalVariables|GetSpawnRotation_Loc) "1,1,1")))
          (bind _output_get_8 (LocalVariables|SetTargetLocation_Loc (Math|Vector|MakeVector (.x (.location _output_get_7)) (.y _spawnpointlocation_c) (.z _spawnpointlocation_c))))
          (return _output_get_8 (LocalVariables|GetSpawnTransform_Loc))))
      (elif (== (LocalVariables|GetRandomInteger_Loc) 2)
        (if (Math|Random|RandomBool)
          (LocalVariables|SetSpawnRotation_Loc "0, 0, 0")
          (bind _output_get_9 (LocalVariables|SetSpawnTransform_Loc (Math|Transform|MakeTransform (Math|Vector|MakeVector (.x _spawnpointlocation_e) (Math|Random|RandomFloatinRange (- (.y _spawnpointlocation_e) _returnvalue_7) (+ (.y _spawnpointlocation_e) _returnvalue_7)) (Variables|Default|GetPedestrianHalfHeight)) (LocalVariables|GetSpawnRotation_Loc) "1,1,1")))
          (bind _output_get_10 (LocalVariables|SetTargetLocation_Loc (Math|Vector|MakeVector (.x _spawnpointlocation_f_2) (.y (.location _output_get_9)) (.z _spawnpointlocation_f_2))))
          (return _output_get_10 (LocalVariables|GetSpawnTransform_Loc))
          (else
            (LocalVariables|SetSpawnRotation_Loc "0, 0, 0")
            (bind _output_get_11 (LocalVariables|SetSpawnTransform_Loc (Math|Transform|MakeTransform (Math|Vector|MakeVector (.x _spawnpointlocation_f) (Math|Random|RandomFloatinRange (- (.y _spawnpointlocation_f) _returnvalue_8) (+ (.y _spawnpointlocation_f) _returnvalue_8)) (Variables|Default|GetPedestrianHalfHeight)) (LocalVariables|GetSpawnRotation_Loc) "1,1,1")))
            (bind _output_get_12 (LocalVariables|SetTargetLocation_Loc (Math|Vector|MakeVector (.x _spawnpointlocation_e_2) (.y (.location _output_get_11)) (.z _spawnpointlocation_e_2))))
            (return _output_get_12 (LocalVariables|GetSpawnTransform_Loc))))
        (elif (== (LocalVariables|GetRandomInteger_Loc) 3)
          (if (Math|Random|RandomBool)
            (LocalVariables|SetSpawnRotation_Loc "0, 0, 0")
            (bind _output_get_13 (LocalVariables|SetSpawnTransform_Loc (Math|Transform|MakeTransform (Math|Vector|MakeVector (.x _spawnpointlocation_g_2) (Math|Random|RandomFloatinRange (- (.y _spawnpointlocation_g_2) _returnvalue_2) (+ (.y _spawnpointlocation_g_2) _returnvalue_2)) (Variables|Default|GetPedestrianHalfHeight)) (LocalVariables|GetSpawnRotation_Loc) "1,1,1")))
            (bind _output_get_14 (LocalVariables|SetTargetLocation_Loc (Math|Vector|MakeVector (.x _spawnpointlocation_h) (.y (.location _output_get_13)) (.z _spawnpointlocation_h))))
            (return _output_get_14 (LocalVariables|GetSpawnTransform_Loc))
            (else
              (LocalVariables|SetSpawnRotation_Loc "0, 0, 0")
              (bind _output_get_15 (LocalVariables|SetSpawnTransform_Loc (Math|Transform|MakeTransform (Math|Vector|MakeVector (.x _spawnpointlocation_h_2) (Math|Random|RandomFloatinRange (- (.y _spawnpointlocation_h_2) _returnvalue_3) (+ (.y _spawnpointlocation_h_2) _returnvalue_3)) (Variables|Default|GetPedestrianHalfHeight)) (LocalVariables|GetSpawnRotation_Loc) "1,1,1")))
              (bind _output_get_16 (LocalVariables|SetTargetLocation_Loc (Math|Vector|MakeVector (.x _spawnpointlocation_g) (.y (.location _output_get_15)) (.z _spawnpointlocation_g))))
              (return _output_get_16 (LocalVariables|GetSpawnTransform_Loc)))))))))

(fn SpawnInitialPedestrians
  (while (<= (Variables|Default|GetPedestrianNumberSpawned) (Variables|Default|GetPedestrianNumberToSpawn))
    (CallFunction|SpawnPedestrian)
    (CallFunction|IncreasePedestrianNumberSpawned))
  (return))

(fn SpawnPedestrian
  (bind _player_ref (Variables|References|GetPlayer_Ref))
  (bind (_targetlocation _spawntransform) (CallFunction|SetPedestrianSpawnTransform))
  (bind _returnvalue (Game|SpawnActorfromClass "/Game/MyContent/Blueprints/Characters/BP_Pedestrian.BP_Pedestrian_C" _spawntransform "AdjustIfPossibleButAlwaysSpawn" 0 (Default|GetRandomTextfromArray _player_ref (Variables|/Game/MyContent/Blueprints/Players/BP_Player.BP_Player_C|GetRecipientFullNames _player_ref)) _targetlocation 0))
  (Utilities|Array|Add (Variables|/Game/MyContent/Blueprints/Players/BP_Player.BP_Player_C|GetPedestrian_Refs (Variables|References|GetPlayer_Ref)) _returnvalue)
  (bind _result (Math|Integer|IncrementInt (Variables|Default|GetPedestrianID))
    (:%20%20
      (bind _output_get (Variables|Default|SetPedestrianID _result))
      (Utilities|Array|Add (Variables|/Script/Engine.Actor|GetTags _returnvalue) (Utilities|String|StringToName (Utilities|String|ToString(Integer) _output_get)))
      (return))))

(fn IncreasePedestrianNumberSpawned
  (bind _result (Math|Integer|IncrementInt (Variables|Default|GetPedestrianNumberSpawned))
    (:%20%20
      (Variables|Default|SetPedestrianNumberSpawned _result)
      (return))))

(fn GetCurrentLevelName
  (bind _returnvalue (Game|GetCurrentLevelName true))
  (bind _output_get (Variables|Default|SetCurrentLevelName _returnvalue))
  (return (Utilities|Enum|Equal(Enum) _output_get (Variables|Default|GetTargetLevelName))))